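; ARC ship actor with four animated, physics-driven landing gears (two back, two front), toggled on BeginPlay and the F key.
; BeginPlay initializes each gear's anim instance, mirroring left-rear bone names for the right.
; Each tick, LGDC sockets set physics constraint targets, with drive strengths and angular limits blended by vertical extension from stiff closed to base values.
; Physics box transforms feed back into the anim instances as override transforms, apparently for Control Rig.
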(event `ABPsInitialization_Event`
  (bind _array (`|MakeArray` "HLB_MAIN_0_DOWN" "HLB_MAIN_1_DOWN" "HLB_MAIN_2_DOWN" "HLB_SUPPORT_0_DOWN" "HLB_SUPPORT_1_DOWN" "HLB_EXTENDER_0_EXT" "HLB_EXTENDER_1_EXT" :!type "Name"))
  (bind _array_2 (`|MakeArray` "HLB_MAIN_0_UP" "HLB_MAIN_1_UP" "HLB_MAIN_2_UP" "HLB_SUPPORT_0_UP" "HLB_SUPPORT_1_UP" "HLB_EXTENDER_0_LCK" "HLB_EXTENDER_1_LCK" :!type "Name"))
  ;[0.08205 0.03103 1 1 60] ABPs initialization
  (`|ExecutionSequence`
    (:`then_0`
      (`self.MirrorRenameArray` _array_2 (`self.LGBR_Up_Bones`) "HLB" "HRB")
      (`self.MirrorRenameArray` _array (`self.LGBR_Down_Bones`) "HLB" "HRB"))
    (:`then_1`
      (for (_array_element _array_index) (`self.AnimInstances`)
        (switch `int` _array_index
          (:`0`
            (bind _asabpi_arc_lgbl (cast `/Game/arc/ARC/LGBL/ABPI_ARC_LGBL` _array_element))
            (`/Game/arc/ARC/ABP_ARC_LG.Initialize` _asabpi_arc_lgbl "/Game/arc/ARC/LGBL/arc_LGBL_OpenAnim.arc_LGBL_OpenAnim" _array_2 _array "HLB_ROOT" (0.0 0.0 0.0)))
          (:`1`
            (bind _asabpi_arc_lgbr (cast `/Game/arc/ARC/LGBR/ABPI_ARC_LGBR` _array_element))
            (`/Game/arc/ARC/ABP_ARC_LG.Initialize` _asabpi_arc_lgbr "/Game/arc/ARC/LGBR/arc_LGBR_OpenAnim.arc_LGBR_OpenAnim" (`self.LGBR_Up_Bones`) (`self.LGBR_Down_Bones`) "HRB_ROOT" (0.0 0.0 0.0)))
          (:`2`
            (bind _asabpi_arc_lgf0 (cast `/Game/arc/ARC/LGF0/ABPI_ARC_LGF0` _array_element))
            (`/Game/arc/ARC/ABP_ARC_LG.Initialize` _asabpi_arc_lgf0 "/Game/arc/ARC/LGF0/arc_LGF0_OpenAnim.arc_LGF0_OpenAnim" (`|MakeArray` "HF0_MIDDLE_UP" "HF0_RIGHT_UP" "HF0_LEFT_UP" :!type "Name") (`|MakeArray` "HF0_MIDDLE_DOWN" "HF0_RIGHT_DOWN" "HF0_LEFT_DOWN" :!type "Name") "HF0_ROOT" (0.0 0.0 0.0)))
          (:`3`
            (bind _asabpi_arc_lgf1 (cast `/Game/arc/ARC/LGF1/ABPI_ARC_LGF1` _array_element))
            (`/Game/arc/ARC/ABP_ARC_LG.Initialize` _asabpi_arc_lgf1 "/Game/arc/ARC/LGF1/arc_LGF1_OpenAnim.arc_LGF1_OpenAnim" (`|MakeArray` "HF1_MIDDLE_UP" "HF1_RIGHT_UP" "HF1_LEFT_UP" :!type "Name") (`|MakeArray` "HF1_MIDDLE_DOWN" "HF1_RIGHT_DOWN" "HF1_LEFT_DOWN" :!type "Name") "HF1_ROOT" (0.0 0.0 0.0))))))))

(event `self.ReceiveBeginPlay`
  (`|ExecutionSequence`
    (:`then_0`
      (set `self.AnimInstances` (`|MakeArray` (`SkeletalMeshComponent.GetAnimInstance` (`self.arc_LGBL_SkeletalMesh`)) (`SkeletalMeshComponent.GetAnimInstance` (`self.arc_LGBR_SkeletalMesh`)) (`SkeletalMeshComponent.GetAnimInstance` (`self.SKM_arc_LGF0`)) (`SkeletalMeshComponent.GetAnimInstance` (`self.SKM_arc_LGF1`)))))
    (:`then_1`
      (`self.ABPsInitialization_Event`))
    (:`then_2`
      (`self.OpenCloseLGs_Event`))))

(event `Key|F`
  (params (Key :type "Key Structure"))
  (:`Pressed`
    (`self.OpenCloseLGs_Event`)))

(event `OpenCloseLGs_Event`
  ;[0.1795 0.2216 1] OpenClose LGs
  (for _array_element (`self.AnimInstances`)
    (bind _asabp_arc_lg (cast `/Game/arc/ARC/ABP_ARC_LG` _array_element))
    (`/Game/arc/ARC/ABP_ARC_LG.OpenCLoseLG` _asabp_arc_lg)
    ;;[0.08333 0.003976 0] wake up physics
    (`KismetSystemLibrary.Delay` 0.1)
    (`PrimitiveComponent.WakeRigidBody` (`self.LGBRBox`) "None")
    (`PrimitiveComponent.WakeRigidBody` (`self.LGBLBox`) "None")
    (`PrimitiveComponent.WakeRigidBody` (`self.LGF0_Box`) "None")
    (`PrimitiveComponent.WakeRigidBody` (`self.LGF1_Box`) "None")))

(event `self.ReceiveTick`
  (params (DeltaSeconds :type "Float (single-precision)"))
  (bind _lgbrdlc (`self.LGBRDLC`))
  (bind _lgbldlc (`self.LGBLDLC`))
  (bind _lgbrdlc_2 (`self.LGBRDLC`))
  (bind _lgf0_dlc (`self.LGF0_DLC`))
  (bind _lgbldlc_2 (`self.LGBLDLC`))
  (bind _lgf1_dlc (`self.LGF1_DLC`))
  (bind _lgf0_dlc_2 (`self.LGF0_DLC`))
  (bind _lgf1_dlc_2 (`self.LGF1_DLC`))
  (bind (_lgdlcvector _lgdrc_x_rotator) (`self.GetLGDCParameters` _lgbrdlc (`self.arc_LGBR_SkeletalMesh`) "LGDC" (`self.ShipBase`) (`self.LGBRDRCObject`)))
  (bind (_lgdlcvector_2 _lgdrc_x_rotator_2) (`self.GetLGDCParameters` _lgbldlc_2 (`self.arc_LGBL_SkeletalMesh`) "LGDC" (`self.ShipBase`) (`self.LGBLDRCObject`)))
  (bind (_lgdlcvector_3 _lgdrc_x_rotator_3 _lgdrc_y_rotator) (`self.GetLGDCParameters` _lgf1_dlc (`self.SKM_arc_LGF1`) "LGDC" (`self.ShipBase`) (`self.LGF1_DRC_Object`)))
  (bind (_lgdlcvector_4 _lgdrc_x_rotator_4 _lgdrc_y_rotator_2) (`self.GetLGDCParameters` _lgf0_dlc_2 (`self.SKM_arc_LGF0`) "LGDC" (`self.ShipBase`) (`self.LGF0_DRC_Object`)))
  (`|ExecutionSequence`
    (:`then_0`
      ;[0 0 0] LGBL
      (`PhysicsConstraintComponent.SetLinearPositionTarget` _lgbldlc_2 _lgdlcvector_2)
      (`PhysicsConstraintComponent.SetAngularOrientationTarget` (`self.LGBLDRC`) _lgdrc_x_rotator_2)
      ;[0 0 0] LGBR
      (`PhysicsConstraintComponent.SetLinearPositionTarget` _lgbrdlc _lgdlcvector)
      (`PhysicsConstraintComponent.SetAngularOrientationTarget` (`self.LGBRDRC`) (`KismetMathLibrary.NegateRotator` _lgdrc_x_rotator))
      ;[0 0 0] LGF0
      (`PhysicsConstraintComponent.SetLinearPositionTarget` _lgf0_dlc_2 _lgdlcvector_4)
      (`PhysicsConstraintComponent.SetAngularOrientationTarget` (`self.LGF0_DRC`) _lgdrc_y_rotator_2)
      ;[0 0 0] LGF1
      (`PhysicsConstraintComponent.SetLinearPositionTarget` _lgf1_dlc _lgdlcvector_3)
      (`PhysicsConstraintComponent.SetAngularOrientationTarget` (`self.LGF1_DRC`) _lgdrc_y_rotator))
    (:`then_1`
      (`self.StatesBehaviour` (`self.LGDCDist` (`self.arc_LGBL_SkeletalMesh`) _lgbldlc) 250.0 300.0 _lgbldlc (`self.LGBLDRC`))
      (`self.StatesBehaviour` (`self.LGDCDist` (`self.arc_LGBR_SkeletalMesh`) _lgbrdlc_2) 250.0 300.0 _lgbrdlc_2 (`self.LGBRDRC`))
      (`self.StatesBehaviourLGF` (`self.LGDCDist` (`self.SKM_arc_LGF0`) _lgf0_dlc) 100.0 300.0 _lgf0_dlc (`self.LGF0_DRC`))
      (`self.StatesBehaviourLGF` (`self.LGDCDist` (`self.SKM_arc_LGF1`) _lgf1_dlc_2) 100.0 300.0 _lgf1_dlc_2 (`self.LGF1_DRC`)))
    (:`then_2`
      (`self.CROverrideLGBL` true (0.0 -66.153613 38.511108) (struct :`Roll` -27.0) (struct :`Roll` 63.0) (`SceneComponent.K2_GetComponentToWorld` (`self.LGBLBox`)) (`self.arc_LGBL_SkeletalMesh`))
      (`self.CROverrideLGBR` true (0.0 66.153613 38.511108) (struct :`Roll` 27.0) (struct :`Pitch` 180.0 :`Roll` 243.0) (`SceneComponent.K2_GetComponentToWorld` (`self.LGBRBox`)) (`self.arc_LGBR_SkeletalMesh`))
      (`self.CROverrideLGF0` true (0.0 0.0 0.0) (struct) (struct :`Roll` 90.0) (`SceneComponent.K2_GetComponentToWorld` (`self.LGF0_Box`)) (`self.SKM_arc_LGF0`))
      (`self.CROverrideLGF1` true (0.0 0.0 0.0) (struct) (struct :`Roll` 90.0) (`SceneComponent.K2_GetComponentToWorld` (`self.LGF1_Box`)) (`self.SKM_arc_LGF1`)))))

(fn `AxisDraw`
  (params (AtPosition :type "Vector Structure") (X :type "Float (double-precision)") (Y :type "Float (double-precision)") (Z :type "Float (double-precision)") (Rotation :type "Rotator Structure"))
  (`self.DrawRay` (`KismetMathLibrary.LinearColor_Red`) AtPosition (`KismetMathLibrary.GreaterGreater_VectorRotator` (500.0 0.0 0.0) Rotation))
  (`self.DrawRay` (`KismetMathLibrary.LinearColor_Green`) AtPosition (`KismetMathLibrary.GreaterGreater_VectorRotator` (0.0 500.0 0.0) Rotation))
  (`self.DrawRay` (`KismetMathLibrary.LinearColor_Blue`) AtPosition (`KismetMathLibrary.GreaterGreater_VectorRotator` (0.0 0.0 500.0) Rotation))
  (return))

(fn `CROverrideLGBL`
  (params (OverrideCR :type Boolean) (InitialTargetPosOffset :type "Vector Structure") (InitialTargetRotOffset :type "Rotator Structure") (CR_RotOffset :type "Rotator Structure") (TargetTransform :type "Transform Structure") (MeshRef :type "SkeletalMeshComponent Object Reference"))
  (bind _rotation (.rotation TargetTransform))
  (bind _asabpi_arc_lgbl (cast `/Game/arc/ARC/LGBL/ABPI_ARC_LGBL` (`SkeletalMeshComponent.GetAnimInstance` MeshRef)))
  (set `/Game/arc/ARC/ABP_ARC_LG.bOverrideTransform` OverrideCR _asabpi_arc_lgbl)
  (if OverrideCR
    (set `/Game/arc/ARC/ABP_ARC_LG.OverrideTransform` (`KismetMathLibrary.MakeTransform` (+ (`KismetMathLibrary.GreaterGreater_VectorRotator` InitialTargetPosOffset (`KismetMathLibrary.ComposeRotators` InitialTargetRotOffset _rotation)) (.location TargetTransform)) (`KismetMathLibrary.ComposeRotators` CR_RotOffset _rotation)) _asabpi_arc_lgbl))
  (return))

(fn `CROverrideLGBR`
  (params (OverrideCR :type Boolean) (InitialTargetPosOffset :type "Vector Structure") (InitialTargetRotOffset :type "Rotator Structure") (CR_RotOffset :type "Rotator Structure") (TargetTransform :type "Transform Structure") (MeshRef :type "SkeletalMeshComponent Object Reference"))
  (bind _rotation (.rotation TargetTransform))
  (bind _asabpi_arc_lgbr (cast `/Game/arc/ARC/LGBR/ABPI_ARC_LGBR` (`SkeletalMeshComponent.GetAnimInstance` MeshRef)))
  (set `/Game/arc/ARC/ABP_ARC_LG.bOverrideTransform` OverrideCR _asabpi_arc_lgbr)
  (if OverrideCR
    (set `/Game/arc/ARC/ABP_ARC_LG.OverrideTransform` (`KismetMathLibrary.MakeTransform` (+ (`KismetMathLibrary.GreaterGreater_VectorRotator` InitialTargetPosOffset (`KismetMathLibrary.ComposeRotators` InitialTargetRotOffset _rotation)) (.location TargetTransform)) (`KismetMathLibrary.ComposeRotators` CR_RotOffset _rotation)) _asabpi_arc_lgbr))
  (return))

(fn `CROverrideLGF0`
  (params (OverrideCR :type Boolean) (InitialTargetPosOffset :type "Vector Structure") (InitialTargetRotOffset :type "Rotator Structure") (CR_RotOffset :type "Rotator Structure") (TargetTransform :type "Transform Structure") (MeshRef :type "SkeletalMeshComponent Object Reference"))
  (bind _rotation (.rotation TargetTransform))
  (bind _asabpi_arc_lgf0 (cast `/Game/arc/ARC/LGF0/ABPI_ARC_LGF0` (`SkeletalMeshComponent.GetAnimInstance` MeshRef)))
  (set `/Game/arc/ARC/ABP_ARC_LG.bOverrideTransform` OverrideCR _asabpi_arc_lgf0)
  (if OverrideCR
    (set `/Game/arc/ARC/ABP_ARC_LG.OverrideTransform` (`KismetMathLibrary.MakeTransform` (+ (`KismetMathLibrary.GreaterGreater_VectorRotator` InitialTargetPosOffset (`KismetMathLibrary.ComposeRotators` InitialTargetRotOffset _rotation)) (.location TargetTransform)) (`KismetMathLibrary.ComposeRotators` CR_RotOffset _rotation)) _asabpi_arc_lgf0))
  (return))

(fn `CROverrideLGF1`
  (params (OverrideCR :type Boolean) (InitialTargetPosOffset :type "Vector Structure") (InitialTargetRotOffset :type "Rotator Structure") (CR_RotOffset :type "Rotator Structure") (TargetTransform :type "Transform Structure") (MeshRef :type "SkeletalMeshComponent Object Reference"))
  (bind _rotation (.rotation TargetTransform))
  (bind _asabpi_arc_lgf1 (cast `/Game/arc/ARC/LGF1/ABPI_ARC_LGF1` (`SkeletalMeshComponent.GetAnimInstance` MeshRef)))
  (set `/Game/arc/ARC/ABP_ARC_LG.bOverrideTransform` OverrideCR _asabpi_arc_lgf1)
  (if OverrideCR
    (set `/Game/arc/ARC/ABP_ARC_LG.OverrideTransform` (`KismetMathLibrary.MakeTransform` (+ (`KismetMathLibrary.GreaterGreater_VectorRotator` InitialTargetPosOffset (`KismetMathLibrary.ComposeRotators` InitialTargetRotOffset _rotation)) (.location TargetTransform)) (`KismetMathLibrary.ComposeRotators` CR_RotOffset _rotation)) _asabpi_arc_lgf1))
  (return))

(fn `DrawRay`
  (params (color :type "LinearColor Structure") (AtPosition :type "Vector Structure") (Vector :type "Vector Structure"))
  (`KismetSystemLibrary.DrawDebugArrow` AtPosition (+ AtPosition Vector) 200.0 color 0.0 4.0)
  (return))

(fn `Get2VectorAngle`
  (params (Vec1 :type "Vector Structure") (Vec2 :type "Vector Structure"))
  (returns (AngleDEG :type "Float (double-precision)"))
  (return (`KismetMathLibrary.DegAcos` (`KismetMathLibrary.Dot_VectorVector` (`KismetMathLibrary.Normal` Vec1) (`KismetMathLibrary.Normal` Vec2)))))

(fn `GetDynamicTransitionParameters`
  (params (`LGRoot-PConstraint_Dist` :type "Float (double-precision)") (TransitionStart :type "Float (double-precision)") (TransitionEnd :type "Float (double-precision)"))
  (returns (PositionLinearStrength :type "Float (double-precision)") (VelocityLinearStrength :type "Float (double-precision)") (AngularOriantationStrength :type "Float (double-precision)") (AngularVelocityStrength :type "Float (double-precision)") (SwingLimit :type "Float (double-precision)"))
  (return (`KismetMathLibrary.MapRangeClamped` `LGRoot-PConstraint_Dist` TransitionStart TransitionEnd 10000.0 (`self.BaseLinearPositionStrength`)) (`KismetMathLibrary.MapRangeClamped` `LGRoot-PConstraint_Dist` TransitionStart TransitionEnd 10.0 (`self.BaseLinearVelocityStrength`)) (`KismetMathLibrary.MapRangeClamped` `LGRoot-PConstraint_Dist` TransitionStart TransitionEnd 100000.0 (`self.BaseAngularOrientationStrength`)) (`KismetMathLibrary.MapRangeClamped` `LGRoot-PConstraint_Dist` TransitionStart TransitionEnd 50.0 (`self.BaseAngularVelocityStrength`)) (`KismetMathLibrary.MapRangeClamped` `LGRoot-PConstraint_Dist` TransitionStart TransitionEnd 110.0 (`self.BaseAngularLimit`))))

(fn `GetLGDCParameters`
  (params (LGDLCRef :type "PhysicsConstraintComponent Object Reference") (SkeletalMeshRef :type "SkeletalMeshComponent Object Reference") (TargetBone :type Name) (ShipBaseRef :type "StaticMeshComponent Object Reference") (LGDRCObjectRef :type "SphereComponent Object Reference"))
  (returns (LGDLCVector :type "Vector Structure") (LGDRC_X_Rotator :type "Rotator Structure") (LGDRC_Y_Rotator :type "Rotator Structure") (LGDRC_Z_Rotator :type "Rotator Structure"))
  (bind _angledeg (`self.Get2VectorAngle` (`KismetMathLibrary.GreaterGreater_VectorRotator` (`KismetMathLibrary.NegateVector` (`KismetMathLibrary.Vector_Right`)) (.rotation (`SceneComponent.GetSocketTransform` SkeletalMeshRef TargetBone "RTS_World"))) (`KismetMathLibrary.GreaterGreater_VectorRotator` (`KismetMathLibrary.Vector_Up`) (`SceneComponent.K2_GetComponentRotation` LGDRCObjectRef))))
  (return (`KismetMathLibrary.LessLess_VectorRotator` (- (.location (`SceneComponent.GetSocketTransform` SkeletalMeshRef TargetBone "RTS_World")) (`SceneComponent.K2_GetComponentLocation` LGDLCRef)) (`SceneComponent.K2_GetComponentRotation` ShipBaseRef)) (`KismetMathLibrary.MakeRotator` _angledeg) (`KismetMathLibrary.MakeRotator` 0.0 _angledeg) (`KismetMathLibrary.MakeRotator` 0.0 0.0 _angledeg)))

(fn `LGDCDist`
  (params (SkeletalMeshRef :type "SkeletalMeshComponent Object Reference") (LGDLCRef :type "PhysicsConstraintComponent Object Reference"))
  (returns (Dist :type "Float (double-precision)"))
  (return (`KismetMathLibrary.Abs` (- (`.Z` (`KismetMathLibrary.BreakVector3f` (`SceneComponent.GetSocketLocation` SkeletalMeshRef "LGDC"))) (`.Z` (`KismetMathLibrary.BreakVector3f` (`SceneComponent.K2_GetComponentLocation` LGDLCRef)))))))

(fn `MirrorRenameArray`
  (params (ArrayToMirror :type "Array of Name") (ArrayToMirrorTo :type "Array of Name") (From :type String) (To :type String))
  (for _array_element ArrayToMirror
    (`KismetArrayLibrary.Array_Add` ArrayToMirrorTo (`KismetStringLibrary.Conv_StringToName` (`KismetStringLibrary.Replace` (`KismetTextLibrary.Conv_TextToString` (`KismetTextLibrary.Conv_NameToText` _array_element)) From To))))
  (return))

(fn `StatesBehaviour`
  (params (Dist :type "Float (double-precision)") (TransitionStart :type "Float (double-precision)") (TransitionEnd :type "Float (double-precision)") (LGDLC :type "PhysicsConstraintComponent Object Reference") (LGDRC :type "PhysicsConstraintComponent Object Reference"))
  (bind (_positionlinearstrength _velocitylinearstrength _angularoriantationstrength _angularvelocitystrength _swinglimit) (`self.GetDynamicTransitionParameters` Dist TransitionStart TransitionEnd))
  (if (< Dist TransitionStart)
    ;[1 0 0] Closed state behaviour
    (`PhysicsConstraintComponent.SetLinearDriveParams` LGDLC 1000000.0 10.0 0.0)
    (`PhysicsConstraintComponent.SetAngularDriveParams` LGDRC 1000000.0 1.0 0.0)
    (`PhysicsConstraintComponent.SetAngularTwistLimit` LGDRC "ACM_Limited" 110.0)
    (else
      ;[0 1 0.04173] Opening behaviour - dynamic transition (/ open state - params clamped)
      (`PhysicsConstraintComponent.SetLinearDriveParams` LGDLC _positionlinearstrength _velocitylinearstrength 0.0)
      (`PhysicsConstraintComponent.SetAngularDriveParams` LGDRC _angularoriantationstrength _angularvelocitystrength 0.0)
      (`PhysicsConstraintComponent.SetAngularTwistLimit` LGDRC "ACM_Limited" _swinglimit)))
  (return))

(fn `StatesBehaviourLGF`
  (params (Dist :type "Float (double-precision)") (TransitionStart :type "Float (double-precision)") (TransitionEnd :type "Float (double-precision)") (LGDLC :type "PhysicsConstraintComponent Object Reference") (LGDRC :type "PhysicsConstraintComponent Object Reference"))
  (bind (_positionlinearstrength _velocitylinearstrength _angularoriantationstrength _angularvelocitystrength _swinglimit) (`self.GetDynamicTransitionParameters` Dist TransitionStart TransitionEnd))
  (if (< Dist TransitionStart)
    ;[1 0 0] Closed state behaviour
    (`PhysicsConstraintComponent.SetLinearDriveParams` LGDLC 1000000.0 10.0 0.0)
    (`PhysicsConstraintComponent.SetAngularDriveParams` LGDRC 1000000.0 1.0 0.0)
    (`PhysicsConstraintComponent.SetAngularSwing2Limit` LGDRC "ACM_Limited" 110.0)
    (else
      ;[0 1 0.04173] Opening behaviour - dynamic transition (/ open state - params clamped)
      (`PhysicsConstraintComponent.SetLinearDriveParams` LGDLC _positionlinearstrength _velocitylinearstrength 0.0)
      (`PhysicsConstraintComponent.SetAngularDriveParams` LGDRC _angularoriantationstrength _angularvelocitystrength 0.0)
      (`PhysicsConstraintComponent.SetAngularSwing2Limit` LGDRC "ACM_Limited" _swinglimit)))
  (return))

(fn `UserConstructionScript`)