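; BP_LG is a helper Blueprint for a ship's LG (apparently landing gear), driving physics constraints as it opens and closes.
; StatesBehaviour holds constraints stiff when closed, then blends drive strengths and twist limit toward base values by clamped distance mapping.
; Helpers measure constraint offset, angle and distance from skeletal mesh sockets, and draw debug axes.
; CROverride passes a target-relative override transform to the ABP_ARC_LGBL anim instance.
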(fn `AxisDraw`
  (params (AtPosition :type "Vector Structure") (X :type "Float (double-precision)") (Y :type "Float (double-precision)") (Z :type "Float (double-precision)") (Rotation :type "Rotator Structure"))
  (`self.DrawRay` (`KismetMathLibrary.LinearColor_Red`) AtPosition (`KismetMathLibrary.GreaterGreater_VectorRotator` (500.0 0.0 0.0) Rotation))
  (`self.DrawRay` (`KismetMathLibrary.LinearColor_Green`) AtPosition (`KismetMathLibrary.GreaterGreater_VectorRotator` (0.0 500.0 0.0) Rotation))
  (`self.DrawRay` (`KismetMathLibrary.LinearColor_Blue`) AtPosition (`KismetMathLibrary.GreaterGreater_VectorRotator` (0.0 0.0 500.0) Rotation))
  (return))

(fn `CROverride`
  (params (OverrideCR :type Boolean) (InitialTargetPosOffset :type "Vector Structure") (InitialTargetRotOffset :type "Rotator Structure") (CR_RotOffset :type "Rotator Structure") (TargetTransform :type "Transform Structure") (MeshRef :type "SkeletalMeshComponent Object Reference"))
  (bind _rotation (.rotation TargetTransform))
  (bind _asabp_arc_lgbl (cast `/Game/arc/ARC/LGBL/ABP_ARC_LGBL` (`SkeletalMeshComponent.GetAnimInstance` MeshRef)))
  (set `/Game/arc/ARC/LGBL/ABP_ARC_LGBL.bOverrideTransform` OverrideCR _asabp_arc_lgbl)
  (if OverrideCR
    (set `/Game/arc/ARC/LGBL/ABP_ARC_LGBL.OverrideTransform` (`KismetMathLibrary.MakeTransform` (+ (`KismetMathLibrary.GreaterGreater_VectorRotator` InitialTargetPosOffset (`KismetMathLibrary.ComposeRotators` InitialTargetRotOffset _rotation)) (.location TargetTransform)) (`KismetMathLibrary.ComposeRotators` CR_RotOffset _rotation)) _asabp_arc_lgbl))
  (return))

(fn `DrawRay`
  (params (color :type "LinearColor Structure") (AtPosition :type "Vector Structure") (Vector :type "Vector Structure"))
  (`KismetSystemLibrary.DrawDebugArrow` AtPosition (+ AtPosition Vector) 200.0 color 0.0 4.0)
  (return))

(fn `Get2VectorAngle`
  (params (Vec1 :type "Vector Structure") (Vec2 :type "Vector Structure"))
  (returns (AngleDEG :type "Float (double-precision)"))
  (return (`KismetMathLibrary.DegAcos` (`KismetMathLibrary.Dot_VectorVector` (`KismetMathLibrary.Normal` Vec1) (`KismetMathLibrary.Normal` Vec2)))))

(fn `GetDynamicTransitionParameters`
  (params (`LGRoot-PConstraint_Dist` :type "Float (double-precision)") (TransitionStart :type "Float (double-precision)") (TransitionEnd :type "Float (double-precision)"))
  (returns (PositionLinearStrength :type "Float (double-precision)") (VelocityLinearStrength :type "Float (double-precision)") (AngularOriantationStrength :type "Float (double-precision)") (AngularVelocityStrength :type "Float (double-precision)") (SwingLimit :type "Float (double-precision)"))
  (return (`KismetMathLibrary.MapRangeClamped` `LGRoot-PConstraint_Dist` TransitionStart TransitionEnd 10000.0 (`self.BaseLinearPositionStrength`)) (`KismetMathLibrary.MapRangeClamped` `LGRoot-PConstraint_Dist` TransitionStart TransitionEnd 10.0 (`self.BaseLinearVelocityStrength`)) (`KismetMathLibrary.MapRangeClamped` `LGRoot-PConstraint_Dist` TransitionStart TransitionEnd 800.0 (`self.BaseAngularOrientationStrength`)) (`KismetMathLibrary.MapRangeClamped` `LGRoot-PConstraint_Dist` TransitionStart TransitionEnd 50.0 (`self.BaseAngularVelocityStrength`)) (`KismetMathLibrary.MapRangeClamped` `LGRoot-PConstraint_Dist` TransitionStart TransitionEnd 110.0 (`self.BaseAngularLimit`))))

(fn `GetLGDCParameters`
  (params (LGDLCRef :type "PhysicsConstraintComponent Object Reference") (SkeletalMeshRef :type "SkeletalMeshComponent Object Reference") (TargetBone :type Name) (ShipBaseRef :type "StaticMeshComponent Object Reference") (LGDRCObjectRef :type "SphereComponent Object Reference"))
  (returns (LGDLCVector :type "Vector Structure") (LGDRCRotator :type "Rotator Structure"))
  (return (`KismetMathLibrary.LessLess_VectorRotator` (- (.location (`SceneComponent.GetSocketTransform` SkeletalMeshRef TargetBone "RTS_World")) (`SceneComponent.K2_GetComponentLocation` LGDLCRef)) (`SceneComponent.K2_GetComponentRotation` ShipBaseRef)) (`KismetMathLibrary.MakeRotator` (`self.Get2VectorAngle` (`KismetMathLibrary.GreaterGreater_VectorRotator` (`KismetMathLibrary.NegateVector` (`KismetMathLibrary.Vector_Right`)) (.rotation (`SceneComponent.GetSocketTransform` SkeletalMeshRef TargetBone "RTS_World"))) (`KismetMathLibrary.GreaterGreater_VectorRotator` (`KismetMathLibrary.Vector_Up`) (`SceneComponent.K2_GetComponentRotation` LGDRCObjectRef))))))

(fn `LGDCDist`
  (params (SkeletalMeshRef :type "SkeletalMeshComponent Object Reference") (LGDLCRef :type "PhysicsConstraintComponent Object Reference"))
  (returns (Dist :type "Float (double-precision)"))
  (return (`KismetMathLibrary.Abs` (- (`.Z` (`KismetMathLibrary.BreakVector3f` (`SceneComponent.GetSocketLocation` SkeletalMeshRef "LGDC"))) (`.Z` (`KismetMathLibrary.BreakVector3f` (`SceneComponent.K2_GetComponentLocation` LGDLCRef)))))))

(fn `SetParams`
  (params (BaseLinearPositionStrength :type "Float (double-precision)") (BaseLinearVelocityStrength :type "Float (double-precision)") (BaseAngularLimit :type "Float (double-precision)") (DynamicTransitionEnd :type "Float (double-precision)") (InitialLGDLCffset :type "Vector Structure") (BaseAngularOrientationStrength :type "Float (double-precision)") (BaseAngularVelocityStrength :type "Float (double-precision)"))
  (set `self.BaseLinearPositionStrength` BaseLinearPositionStrength)
  (set `self.BaseLinearVelocityStrength` BaseLinearVelocityStrength)
  (set `self.BaseAngularLimit` BaseAngularLimit)
  (set `self.BaseAngularLimit` DynamicTransitionEnd)
  (set `self.InitialLGDLCffset` InitialLGDLCffset)
  (set `self.BaseAngularOrientationStrength` BaseAngularOrientationStrength)
  (set `self.BaseAngularVelocityStrength` BaseAngularVelocityStrength)
  (return))

(fn `StatesBehaviour`
  (params (Dist :type "Float (double-precision)") (TransitionStart :type "Float (double-precision)") (TransitionEnd :type "Float (double-precision)") (LGDLC :type "PhysicsConstraintComponent Object Reference") (LGDRC :type "PhysicsConstraintComponent Object Reference"))
  (bind (_positionlinearstrength _velocitylinearstrength _angularoriantationstrength _angularvelocitystrength _swinglimit) (`self.GetDynamicTransitionParameters` Dist TransitionStart TransitionEnd))
  (if (< Dist TransitionStart)
    ;[1 0 0] Closed state behaviour
    (`PhysicsConstraintComponent.SetLinearDriveParams` LGDLC 1000000.0 10.0 0.0)
    (`PhysicsConstraintComponent.SetAngularDriveParams` LGDRC 1000000.0 1.0 0.0)
    (`PhysicsConstraintComponent.SetAngularTwistLimit` LGDRC "ACM_Limited" 110.0)
    (else
      ;[0 1 0.04173] Opening behaviour - dynamic transition (/ open state - params clamped)
      (`PhysicsConstraintComponent.SetLinearDriveParams` LGDLC _positionlinearstrength _velocitylinearstrength 0.0)
      (`PhysicsConstraintComponent.SetAngularDriveParams` LGDRC _angularoriantationstrength _angularvelocitystrength 0.0)
      (`PhysicsConstraintComponent.SetAngularTwistLimit` LGDRC "ACM_Limited" _swinglimit)))
  (return))