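; Landing gear test actor that toggles opening and closing through ABP_ARC_LGF0V2 on F, and 1.5 seconds after BeginPlay.
; Each Tick, root socket-to-constraint vertical distance sets the physics constraint's targets and Z limit, blending drive strength and swing between closed and open states.
; The Box's transform, pitched 90 degrees, overrides the AnimBP transform.
; Toggling nudges the Box as a constraint workaround.
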(event `Key|F`
  (params (Key :type "Key Structure"))
  (bind _box (`self.Box`))
  ;[1 0.01752 0] manual lg opening
  (:`Pressed`
    (bind _asabp_arc_lgf0v2 (cast `/Game/arc/ARC_LGF0V2/ABP_ARC_LGF0V2` (`SkeletalMeshComponent.GetAnimInstance` (`self.LGSkeletalMesh`)) :!label _label))
    (`/Game/arc/ARC_LGF0V2/ABP_ARC_LGF0V2.OpenCLoseLG` _asabp_arc_lgf0v2)
    ;[0 0 0] fix for physics constraint
    (`SceneComponent.K2_SetWorldLocation` _box (+ (`SceneComponent.K2_GetComponentLocation` _box) (0.5 0.0 0.0)) false false)))

(event `self.ReceiveBeginPlay`
  (`|ExecutionSequence`
    (:`then_0`
      (bind _asabp_arc_lgf0v2 (cast `/Game/arc/ARC_LGF0V2/ABP_ARC_LGF0V2` (`SkeletalMeshComponent.GetAnimInstance` (`self.LGSkeletalMesh`))))
      (set `/Game/arc/ARC_LGF0V2/ABP_ARC_LGF0V2.bOverrideTransform` false _asabp_arc_lgf0v2))
    (:`then_1`
      (`KismetSystemLibrary.Delay` 1.5)
      (goto _label))))

(event `self.ReceiveTick`
  (params (DeltaSeconds :type "Float (single-precision)"))
  (bind _lgdynamicconstraint (`self.LGDynamicConstraint`))
  (bind _lgskeletalmesh (`self.LGSkeletalMesh`))
  (bind _lgdynamicconstraint_2 (`self.LGDynamicConstraint`))
  (bind _returnvalue (`KismetMathLibrary.Abs` (- (`.Z` (`KismetMathLibrary.BreakVector3f` (`SceneComponent.GetSocketLocation` (`self.LGSkeletalMesh`) "HF0_ROOT_LCK"))) (`.Z` (`KismetMathLibrary.BreakVector3f` (`SceneComponent.K2_GetComponentLocation` (`self.LGDynamicConstraint`)))))))
  (bind (_positionstrength _velocitystrength _swinglimit) (`self.GetDynamicTransitionParameters` _returnvalue))
  (bind _returnvalue_2 (`KismetMathLibrary.MakeVector` 0.0 0.0 _returnvalue))
  (`|ExecutionSequence`
    (:`then_0`
      (if (< _returnvalue 100.0)
        ;[0 0.1029 1] closed state behaviour
        (`PhysicsConstraintComponent.SetLinearDriveParams` _lgdynamicconstraint 100000.0 0.0 0.0)
        (`PhysicsConstraintComponent.SetAngularSwing2Limit` _lgdynamicconstraint "ACM_Limited" 0.0)
        (elif (< _returnvalue (`self.DynamicTransition`))
          ;[0 0.1029 1] Opening behaviour - dynamic transition
          (`PhysicsConstraintComponent.SetLinearDriveParams` _lgdynamicconstraint_2 _positionstrength _velocitystrength 0.0)
          (`PhysicsConstraintComponent.SetAngularSwing2Limit` _lgdynamicconstraint_2 "ACM_Limited" _swinglimit)
          (else
            ;[0 0.1029 1] Open state behaviour
            (`PhysicsConstraintComponent.SetLinearDriveParams` _lgdynamicconstraint_2 (`self.BaseLinearPositionStrength`) (`self.BaseLinearVelocityStrength`) 0.0)
            (`PhysicsConstraintComponent.SetAngularSwing2Limit` _lgdynamicconstraint_2 "ACM_Limited" (`self.BaseAngularLimit`))))))
    (:`then_1`
      (`PhysicsConstraintComponent.SetLinearPositionTarget` _lgdynamicconstraint _returnvalue_2)
      (`PhysicsConstraintComponent.SetLinearVelocityTarget` _lgdynamicconstraint _returnvalue_2)
      (`PhysicsConstraintComponent.SetLinearZLimit` _lgdynamicconstraint "LCM_Limited" _returnvalue)
      (`|ExecutionSequence`
        (:`then_0`
          (bind _asabp_arc_lgf0v2 (cast `/Game/arc/ARC_LGF0V2/ABP_ARC_LGF0V2` (`SkeletalMeshComponent.GetAnimInstance` _lgskeletalmesh)))
          (set `/Game/arc/ARC_LGF0V2/ABP_ARC_LGF0V2.bOverrideTransform` true _asabp_arc_lgf0v2))
        (:`then_1`
          (bind _asabp_arc_lgf0v2_2 (cast `/Game/arc/ARC_LGF0V2/ABP_ARC_LGF0V2` (`SkeletalMeshComponent.GetAnimInstance` _lgskeletalmesh)))
          (set `/Game/arc/ARC_LGF0V2/ABP_ARC_LGF0V2.OverrideTransform` (`KismetMathLibrary.MakeTransform` (.location (`SceneComponent.K2_GetComponentToWorld` (`self.Box`))) (`KismetMathLibrary.ComposeRotators` (struct :`Roll` 90.0) (.rotation (`SceneComponent.K2_GetComponentToWorld` (`self.Box`))))) _asabp_arc_lgf0v2_2))))))

(fn `GetDynamicTransitionParameters`
  (params (`LGRoot-PConstraint_Dist` :type "Float (double-precision)"))
  (returns (PositionStrength :type "Float (double-precision)") (VelocityStrength :type "Float (double-precision)") (SwingLimit :type "Float (double-precision)"))
  (bind _dynamictransition (`self.DynamicTransition`))
  (return (`KismetMathLibrary.MapRangeClamped` `LGRoot-PConstraint_Dist` 100.0 _dynamictransition 6000.0 (`self.BaseLinearPositionStrength`)) (`KismetMathLibrary.MapRangeClamped` `LGRoot-PConstraint_Dist` 100.0 _dynamictransition 0.0 (`self.BaseLinearVelocityStrength`)) (`KismetMathLibrary.MapRangeClamped` `LGRoot-PConstraint_Dist` 100.0 _dynamictransition 0.0 (`self.BaseAngularLimit`))))

(fn `UserConstructionScript`)