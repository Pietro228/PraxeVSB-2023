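; BP_Furnace_FIXED is a furnace that smelts items placed inside it once lit.
; Lighting happens once, setting IsOnFire, spawning fire Niagara and playing forge audio.
; Box overlaps track actors and first tags; entry while burning restarts a timeline, stopped if the latest actor leaves.
; On finish, it calls Smelted on BP_Ingot actors and, given Flour and WaterBucket tags, spawns BP_MagicRock and destroys tracked actors.
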(event `/Game/Blueprints/Interfaces/SpellReactionInterface.LightOnFire`
  (`/Engine/EditorBlueprintResources/StandardMacros.DoOnce` false :!label _label
    (:`Completed`
      (set `self.IsOnFire` true)
      (`NiagaraFunctionLibrary.SpawnSystemAtLocation` "/Game/Niagara/NPS_Fire.NPS_Fire" (`self.K2_GetActorLocation`))
      (`KismetSystemLibrary.Delay` 0.2)
      (`AudioComponent.Play` (`self.forge_Cue`) 0.0))))

(event `/Game/Blueprints/Interfaces/ActionTriggerableActorInterface.ActionTriggered`
  (goto _label))

(event `self.Box.OnComponentBeginOverlap`
  (params (OverlappedComponent :type "PrimitiveComponent Object Reference") (OtherActor :type "Actor Object Reference") (OtherComp :type "PrimitiveComponent Object Reference") (OtherBodyIndex :type Integer) (bFromSweep :type Boolean) (SweepResult :type "HitResult Structure (by ref)"))
  (bind _actorssmelting0 (`self.ActorsSmelting0`))
  (bind _actorssmelting (`self.ActorsSmelting`))
  (bind _tags (`Actor.Tags` OtherActor))
  (bind (_returnvalue_location _returnvalue_rotation) (`KismetMathLibrary.BreakTransform` (`SceneComponent.K2_GetComponentToWorld` (`self.Box`))))
  (bind _output (`|GetArrayItem` _actorssmelting0))
  (`KismetArrayLibrary.Array_Add` (`self.ActorsSmelting0`) OtherActor)
  (if (`KismetArrayLibrary.Array_IsNotEmpty` _tags)
    (`KismetArrayLibrary.Array_AddUnique` (`self.ActorsSmelting`) (`|GetArrayItem` _tags)))
  (set `self.ActorToSmelt` OtherActor)
  (if (`self.IsOnFire`)
    (`Timeline|Timeline` :!via `PlayFromStart` :!label _label_2
      (:`Finished`
        (`|ExecutionSequence`
          (:`then_0`
            (bind _asbp_ingot (cast `/Game/Blueprints/Actors/BP_Ingot` OtherActor))
            (`/Game/Blueprints/Actors/BP_Ingot.Smelted` _asbp_ingot))
          (:`then_1`
            (if (and (`KismetArrayLibrary.Array_Contains` _actorssmelting "Flour") (`KismetArrayLibrary.Array_Contains` _actorssmelting "WaterBucket"))
              (`|SpawnActorFromClass` "/Game/Blueprints/Actors/BP_MagicRock.BP_MagicRock_C" (`KismetMathLibrary.MakeTransform` (- _returnvalue_location (0.0 0.0 0.0)) _returnvalue_rotation) "Undefined" "OverrideRootScale" null "NewEnumerator5" null)
              (for _ (range (+ (`KismetArrayLibrary.Array_Length` _actorssmelting0) 1))
                (`/Engine/EditorBlueprintResources/StandardMacros.IsValid` _output
                  (:`Is Valid`
                    (`self.K2_DestroyActor` _output)))))))))))

(event `self.Box.OnComponentEndOverlap`
  (params (OverlappedComponent :type "PrimitiveComponent Object Reference") (OtherActor :type "Actor Object Reference") (OtherComp :type "PrimitiveComponent Object Reference") (OtherBodyIndex :type Integer))
  (`KismetArrayLibrary.Array_RemoveItem` (`self.ActorsSmelting0`) OtherActor)
  (if (`KismetArrayLibrary.Array_IsNotEmpty` (`Actor.Tags` (stale `self.Box.OnComponentBeginOverlap` OtherActor)))
    (`KismetArrayLibrary.Array_RemoveItem` (`self.ActorsSmelting`) (`|GetArrayItem` (`Actor.Tags` OtherActor))))
  (if (== OtherActor (`self.ActorToSmelt`))
    (goto _label_2 :!via `Stop`)))

(fn `UserConstructionScript`)