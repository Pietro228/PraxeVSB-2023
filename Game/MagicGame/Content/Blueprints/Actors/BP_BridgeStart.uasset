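; BP_BridgeStart is an actor that triggers a bridge action once all pressure plates in the level are activated.
; On BeginPlay it counts every BP_PressurePlate to set the required total.
; StartBridge compares ActivatedPressurePlates to that total and, on a match, calls Trigger on its BPActionComponent through a DoOnce, which resets whenever the counts differ.
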(event `self.ReceiveBeginPlay`
  (bind _outactors (`GameplayStatics.GetAllActorsOfClass` "/Game/Blueprints/Actors/BP_PressurePlate.BP_PressurePlate_C"))
  (set `self.NumOfPressurePlates` (`KismetArrayLibrary.Array_Length` _outactors)))

(event `StartBridge`
  (if (== (`self.ActivatedPressurePlates`) (`self.NumOfPressurePlates`))
    (`/Engine/EditorBlueprintResources/StandardMacros.DoOnce` false :!label _label
      (:`Completed`
        (`/Game/Blueprints/Components/BP_ActionComponent.Trigger` (`self.BP_ActionComponent`))))
    (else
      (goto _label :!via `Reset`))))

(fn `UserConstructionScript`)