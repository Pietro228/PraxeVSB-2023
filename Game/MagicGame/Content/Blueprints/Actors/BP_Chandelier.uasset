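; BP_Chandelier is a chandelier actor whose point light flickers like fire.
; The construction script sets the light to MaxIntensity.
; From BeginPlay, it picks a random intensity in the top quarter below MaxIntensity and blends to it with FireLerpTimeline, then repeats when the timeline finishes for an endless flicker.
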(event `self.ReceiveBeginPlay`
  (`self.NewFireIntensity`))

(event `NewFireIntensity`
  (bind _maxintensity (`self.MaxIntensity`))
  (set `self.LastFireIntensity` (`LightComponentBase.Intensity` (`self.PointLight`)))
  (set `self.FireIntensity` (`KismetMathLibrary.RandomFloatInRange` (- _maxintensity (/ _maxintensity 4.0)) _maxintensity))
  (bind (_direction _lerp) (`Timeline|FireLerpTimeline` :!via `PlayFromStart`)
    (:`Update`
      (`LightComponent.SetIntensity` (`self.PointLight`) (`KismetMathLibrary.Lerp` (`self.LastFireIntensity`) (`self.FireIntensity`) _lerp)))
    (:`Finished`
      (`self.NewFireIntensity`))))

(fn `UserConstructionScript`
  (`LightComponent.SetIntensity` (`self.PointLight`) (`self.MaxIntensity`)))