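; BP_Cobweb_2 is a cobweb actor that burns away once set alight through LightonFire.
; The construction script gives the plane a dynamic material using the configurable WebTexture.
; LightonFire runs once, attaching Niagara fire and playing a timeline that drives the material's Burned parameter alongside a one-shot sound.
; When the timeline finishes, it removes the plane, zeroes the fire amount, then destroys the Bound actor and itself.
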(event `/Game/Blueprints/Interfaces/SpellReactionInterface.LightOnFire`
  (`/Engine/EditorBlueprintResources/StandardMacros.DoOnce` false
    (:`Completed`
      (bind _returnvalue (`NiagaraFunctionLibrary.SpawnSystemAttached` "/Game/Niagara/NPS_Fire.NPS_Fire" (`self.NPS_Root`) "None" (0.0 0.0 0.0) (struct) "KeepRelativeOffset"))
      (bind (_direction _alpha) (`Timeline|BurnTimeline`)
        (:`Update`
          (`MeshComponent.SetScalarParameterValueOnMaterials` (`self.Plane`) "Burned" _alpha)
          (`/Engine/EditorBlueprintResources/StandardMacros.DoOnce` false
            (:`Completed`
              (`AudioComponent.Play` (`self.fire_cobweb_Cue`) 0.0))))
        (:`Finished`
          (`ActorComponent.K2_DestroyComponent` (`self.Plane`))
          (`NiagaraComponent.SetVariableFloat` _returnvalue "Amount" 0.0)
          (`KismetSystemLibrary.Delay` 0.1)
          (`self.K2_DestroyActor` (`self.Bound`))
          (`self.K2_DestroyActor`))))))

(fn `UserConstructionScript`
  (bind _returnvalue (`KismetMaterialLibrary.CreateDynamicMaterialInstance` "/Game/Models/Assets/Materials/M_web_variance_one_Mat.M_web_variance_one_Mat"))
  (`MaterialInstanceDynamic.SetTextureParameterValue` _returnvalue "Pavucina" (`self.WebTexture`))
  (`PrimitiveComponent.SetMaterial` (`self.Plane`) 0 _returnvalue))