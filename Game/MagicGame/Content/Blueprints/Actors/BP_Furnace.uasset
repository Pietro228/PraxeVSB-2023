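; BP_Furnace is a furnace actor that can be lit once and then smelts ingots that touch it.
; A LightonFire or ActionTriggered event passes through a DoOnce that sets IsOnFire, spawns a Niagara fire effect and, after a short delay, plays the forge cue.
; While lit, any BP_Ingot that begins overlapping its Box has Smelted called on it.
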(event `/Game/Blueprints/Interfaces/SpellReactionInterface.LightOnFire`
  (`/Engine/EditorBlueprintResources/StandardMacros.DoOnce` false :!label _label
    (:`Completed`
      (set `self.IsOnFire` true)
      (`NiagaraFunctionLibrary.SpawnSystemAtLocation` "/Game/Niagara/NPS_Fire.NPS_Fire" (`self.K2_GetActorLocation`))
      (`KismetSystemLibrary.Delay` 0.2)
      (`AudioComponent.Play` (`self.forge_Cue`) 0.0))))

(event `/Game/Blueprints/Interfaces/ActionTriggerableActorInterface.ActionTriggered`
  (goto _label))

(event `self.Box.OnComponentBeginOverlap`
  (params (OverlappedComponent :type "PrimitiveComponent Object Reference") (OtherActor :type "Actor Object Reference") (OtherComp :type "PrimitiveComponent Object Reference") (OtherBodyIndex :type Integer) (bFromSweep :type Boolean) (SweepResult :type "HitResult Structure (by ref)"))
  (if (`self.IsOnFire`)
    (bind _asbp_ingot (cast `/Game/Blueprints/Actors/BP_Ingot` OtherActor))
    (`/Game/Blueprints/Actors/BP_Ingot.Smelted` _asbp_ingot)))

(fn `UserConstructionScript`)