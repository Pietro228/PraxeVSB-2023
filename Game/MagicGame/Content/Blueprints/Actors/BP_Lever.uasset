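; BP_Lever is a lever actor that fires separate on and off actions based on the handle's rotation.
; Each tick it checks the LeverHandle's relative roll against positive and negative thresholds, triggering the matching BPActionComponent and playing LeverCue.
; DoOnce gates keep each side from repeating and reset when the handle returns to the middle range.
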(event `self.ReceiveTick`
  (params (DeltaSeconds :type "Float (single-precision)"))
  (bind _relativerotation_roll (`KismetMathLibrary.BreakRotator` (`SceneComponent.RelativeRotation` (`self.LeverHandle`))))
  (if (> _relativerotation_roll 30.0)
    (`/Engine/EditorBlueprintResources/StandardMacros.DoOnce` false :!label _label
      (:`Completed`
        (`/Game/Blueprints/Components/BP_ActionComponent.Trigger` (`self.BP_ActionComponent_On`))
        (`KismetSystemLibrary.PrintString` "On")))
    (elif (< _relativerotation_roll -30.0)
      (`/Engine/EditorBlueprintResources/StandardMacros.DoOnce` false :!label _label_2
        (:`Completed`
          (`/Game/Blueprints/Components/BP_ActionComponent.Trigger` (`self.BP_ActionComponent_Off`))
          (`KismetSystemLibrary.PrintString` "Off")))
      (else
        (`|ExecutionSequence`
          (:`then_0`
            (goto _label :!via `Reset`))
          (:`then_1`
            (goto _label_2 :!via `Reset`))))))
  (`AudioComponent.Play` (`self.LeverCue`) 0.0))

(fn `UserConstructionScript`)