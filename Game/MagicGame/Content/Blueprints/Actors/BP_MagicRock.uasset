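; BP_MagicRock is a spell pickup that, when interacted with, unlocks its Spell in the player's Kodex and destroys itself.
; The construction script picks the mesh from the Spell value, adding a second stone for Telekinesis and showing a decal for Bread.
; When Spell is the first value, Tick plays a Levitation timeline that raises and tilts both meshes on separate alpha tracks.
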(event `self.ReceiveTick`
  (params (DeltaSeconds :type "Float (single-precision)"))
  (if (== (`self.Spell`) 0)
    (bind (_direction _alpha0 _alpha1) (`Timeline|Levitation`)
      (:`Update`
        (bind _returnvalue (`KismetMathLibrary.Lerp` 0.0 5.0 _alpha0))
        (`SceneComponent.K2_SetRelativeLocationAndRotation` (`self.MagicRock`) (`KismetMathLibrary.MakeVector` 0.0 0.0 _returnvalue) (`KismetMathLibrary.MakeRotator` (* _returnvalue 3.0) (* _returnvalue 5.0)) false false)
        (bind _returnvalue_2 (`KismetMathLibrary.Lerp` 0.0 5.0 _alpha1))
        (`SceneComponent.K2_SetRelativeLocationAndRotation` (`self.MagicRock1`) (`KismetMathLibrary.MakeVector` 0.0 0.0 _returnvalue_2) (`KismetMathLibrary.MakeRotator` (* _returnvalue_2 2.0) (* _returnvalue_2 1.5)) false false)))))

(event `/Game/Blueprints/Interfaces/InteractableActorInterface.Interacted`
  (params (Hit :type "HitResult Structure"))
  (bind _asbp_player (cast `/Game/Blueprints/Characters/BP_Player` (`GameplayStatics.GetPlayerCharacter` 0)))
  (`/Game/Blueprints/Actors/BP_Kodex.UnlockSpell` (`/Game/Blueprints/Characters/BP_Player.Kodex` _asbp_player) (`self.Spell`))
  (`self.K2_DestroyActor`))

(fn `UserConstructionScript`
  (bind _returnvalue (select `/Game/Blueprints/Utilities/Enums/ESpellType` (`self.Spell`) :`NewEnumerator0` "/Game/Models/Assets/telekinesesStoneLeft.telekinesesStoneLeft" :`NewEnumerator3` "/Game/Models/Assets/lucerna_lightspell.lucerna_lightspell" :`NewEnumerator1` "/Game/Models/Assets/CANDLENASUB.CANDLENASUB" :`NewEnumerator5` "/Game/Models/Assets/Bread.Bread" :!type "StaticMesh Object Reference"))
  (if (== _returnvalue "/Game/Models/Assets/telekinesesStoneLeft.telekinesesStoneLeft")
    (`StaticMeshComponent.SetStaticMesh` (`self.MagicRock1`) "/Game/Models/Assets/telekinesesStoneRight.telekinesesStoneRight"))
  (`StaticMeshComponent.SetStaticMesh` (`self.MagicRock`) _returnvalue)
  (if (== _returnvalue "/Game/Models/Assets/Bread.Bread")
    (`SceneComponent.SetVisibility` (`self.Decal`) true false)))