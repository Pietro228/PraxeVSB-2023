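; BP_MrizeDoor is a breakable door that loses HP when its Box collision is hit.
; Each hit subtracts the impulse magnitude, with a DoOnce reset after a one-second delay to throttle damage.
; When HP drops below zero, the Mrize component simulates physics, Box collision turns off, OnDoorBroken fires, and the Bound nav area switches to default.
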(event `self.Box.OnComponentHit`
  (params (HitComponent :type "PrimitiveComponent Object Reference") (OtherActor :type "Actor Object Reference") (OtherComp :type "PrimitiveComponent Object Reference") (NormalImpulse :type "Vector Structure") (Hit :type "HitResult Structure (by ref)"))
  (`/Engine/EditorBlueprintResources/StandardMacros.DoOnce` false :!label _label
    (:`Completed`
      (`|ExecutionSequence`
        (:`then_0`
          (bind _output_get (set `self.HP` (- (stale _output_get) (`KismetMathLibrary.VSize` NormalImpulse))))
          (if (< _output_get 0.0)
            (`PrimitiveComponent.SetSimulatePhysics` (`self.Mrize`) true)
            (`PrimitiveComponent.SetCollisionEnabled` (`self.Box`) "NoCollision")
            (`self.OnDoorBroken`)
            (`NavModifierVolume.SetAreaClass` (`self.Bound`) "/Script/NavigationSystem.NavArea_Default")))
        (:`then_1`
          (`KismetSystemLibrary.Delay` 1.0)
          (goto _label :!via `Reset`))))))

(fn `UserConstructionScript`)