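; Pitcher prop built on a Geometry Collection, given a random yaw at BeginPlay for placement variety.
; Component hits play a sound cue through a DoOnce gate, with its volume multiplier set in the construction script from a variable.
; A second DoOnce, never reset itself, re-arms the sound gate only once, after a short delay from the first hit.
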(event `self.ReceiveBeginPlay`
  (`SceneComponent.K2_SetWorldRotation` (`self.GeometryCollectionComponent`) (`KismetMathLibrary.MakeRotator` 0.0 0.0 (`KismetMathLibrary.RandomFloatInRange` 0.0 360.0)) false false))

(event `self.GeometryCollectionComponent.OnComponentHit`
  (params (HitComponent :type "PrimitiveComponent Object Reference") (OtherActor :type "Actor Object Reference") (OtherComp :type "PrimitiveComponent Object Reference") (NormalImpulse :type "Vector Structure") (Hit :type "HitResult Structure (by ref)"))
  (`|ExecutionSequence`
    (:`then_0`
      (`/Engine/EditorBlueprintResources/StandardMacros.DoOnce` false :!label _label
        (:`Completed`
          (`AudioComponent.Play` (`self.NewSoundCue`) 0.1))))
    (:`then_1`
      (`/Engine/EditorBlueprintResources/StandardMacros.DoOnce` false
        (:`Completed`
          (`KismetSystemLibrary.Delay` 3.0)
          (goto _label :!via `Reset`))))))

(fn `UserConstructionScript`
  (`AudioComponent.SetVolumeMultiplier` (`self.NewSoundCue`) (`self.Vol`)))