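; BP_Wand is the player's spell wand, toggling Telekinesis or Light on use; Fire and Freeze are empty stubs.
; UseSpell raycasts from the camera and CastSpell dispatches on the current spell, while ChargeWand drives the tip's particle rate and color.
; Light fades a point light by timeline.
; Telekinesis pulls physics objects in through a PhysicsHandle, holds them until timeout or toggle-off, then releases, launching them forward on alternative use.
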(event `self.ReceiveTick`
  (params (DeltaSeconds :type "Float (single-precision)"))
  ;[0.5938 0 1] Tick
  (if (`self.TelekinesisActive`)
    (`PhysicsHandleComponent.SetTargetLocation` (`self.PhysicsHandle`) (`SceneComponent.K2_GetComponentLocation` (`self.GrabLocation`)))))

(event `self.ReceiveBeginPlay`
  ;[0.5 0 1] Begin Play
)

(event `SpellLight`
  (params (Hit :type "HitResult Structure"))
  (bind _wasactivated (`self.WasActivated`))
  ;[0 0.4375 1] Hadouken Spell
  (`self.ChargeWand` _wasactivated)
  (if _wasactivated
    (bind (_direction _alpha) (`Timeline|SpellLightIntesityTimeline` :!label _label)
      (:`Update`
        (`LightComponent.SetIntensity` (`self.PointLight`) (`KismetMathLibrary.Lerp` 0.0 3000.0 _alpha))))
    (else
      (goto _label :!via `Reverse`))))

(event `SpellTelekinesis`
  (params (Hit :type "HitResult Structure"))
  (bind (_bblockinghit _binitialoverlap _time _distance _location _impactpoint _normal _impactnormal _physmat _hitactor _hitcomponent) (`GameplayStatics.BreakHitResult` Hit))
  ;[0.6406 0 1] Telekinesis Grab
  (if (`self.WasActivated`)
    (if _bblockinghit
      (bind _output_get (set `self.SpellTelekinesisHit Component` _hitcomponent))
      (`PhysicsHandleComponent.GrabComponentAtLocation` (`self.PhysicsHandle`) _output_get "None" _location)
      (`self.ChargeWand` true)
      (bind (_direction _location_2) (`Timeline|FliToWand` :!via `PlayFromStart`)
        (:`Update`
          (`PhysicsHandleComponent.SetTargetLocation` (`self.PhysicsHandle`) (`KismetMathLibrary.VLerp` _location (`SceneComponent.K2_GetComponentLocation` (`self.GrabLocation`)) _location_2)))
        (:`Finished`
          (set `self.TelekinesisActive` true)
          (`Timeline|StopTelekinesisTimeline` :!via `PlayFromStart`
            (:`Finished`
              (set `self.TelekinesisActive` false :!label _label_2)
              (`self.ChargeWand` false)
              (`PhysicsHandleComponent.ReleaseComponent` (`self.PhysicsHandle`))
              (if (`self.Alternative Spell Use`)
                (`PrimitiveComponent.AddImpulse` (`self.SpellTelekinesisHit Component`) (* (`SceneComponent.GetForwardVector` (`/Game/Blueprints/Characters/BP_Player.FirstPersonCamera` (`self.Player`))) 1000) "None" true))))))
      (else
        (set `self.WasActivated` false)))
    (else
      (`TimelineComponent.Stop` (`self.StopTelekinesisTimeline`))
      (goto _label_2))))

(event `SpellFire`
  (params (Hit :type "HitResult Structure")))

(event `SpellFreeze`
  (params (Hit :type "HitResult Structure")))

(event `UseSpell`
  (params (AlternativeUse :type Boolean))
  ;[1 0.8438 0] Using spell
  (set `self.Alternative Spell Use` AlternativeUse)
  (bind _output_get (set `self.WasActivated` (not (stale _output_get))))
  (bind _hit (`/Game/Blueprints/Utilities/BlueprintUtilities/BPFL_qol.Raycast` (`self.Camera`) 1000.0 "ObjectTypeQuery4" "Persistent"))
  (`self.CastSpell` (`self.CurrentSpell`) _hit))

(fn `CastSpell`
  (params (SpellType :type "/Game/Blueprints/Utilities/Enums/ESpellType Enum" :default "NewEnumerator0") (HitObject :type "HitResult Structure"))
  (switch `/Game/Blueprints/Utilities/Enums/ESpellType` SpellType
    (:`NewEnumerator0`
      (`self.SpellTelekinesis` HitObject))
    (:`NewEnumerator3`
      (`self.SpellLight` HitObject))
    (:`NewEnumerator1`
      (`self.SpellFire` HitObject))
    (:`NewEnumerator2`
      (`self.SpellFreeze` HitObject))))

(fn `ChargeWand`
  (params (bIsCharged :type Boolean))
  (locals (BaseSpawnRate :type "Float (double-precision)" :default 1000.0))
  (bind _wandtip (`self.WandTip`))
  (`NiagaraComponent.SetVariableFloat` _wandtip "user.SpawnRate" (`KismetMathLibrary.SelectFloat` (`local.BaseSpawnRate`) 0.0 bIsCharged))
  (`NiagaraComponent.SetVariableLinearColor` _wandtip "user.ChargeColor" (`|GetArrayItem` (`self.SpellCollors`) (`KismetMathLibrary.Conv_ByteToInt` (`self.CurrentSpell`)))))

(fn `Initialize`
  (params (Player :type "/Game/Blueprints/Characters/BP_Player Object Reference") (Camera :type "SceneComponent Object Reference"))
  (bind _output_get (set `self.Player` Player))
  (set `self.BaseRotation` (.rotation (`SceneComponent.GetRelativeTransform` (`/Game/Blueprints/Characters/BP_Player.BP_Wand` _output_get))))
  (set `self.Camera` Camera)
  (return))

(fn `ResetSpells`
  (bind _hud (`/Game/Blueprints/Characters/BP_Player.HUD` (`self.Player`)))
  (if (`self.WasActivated`)
    (if (`|EnumInequality` (`self.CurrentSpell`) "NewEnumerator0")
      (`self.SpellTelekinesis` (struct))
      (`TimelineComponent.Stop` (`self.StopTelekinesisTimeline`))
      (`Widget.SetVisibility` (`/Game/Widgets/WBP_HUD.Telekinesis` _hud) "Collapsed")
      (elif (`|EnumInequality` (`self.CurrentSpell`) "NewEnumerator3")
        (`self.SpellLight` (struct))
        (`Widget.SetVisibility` (`/Game/Widgets/WBP_HUD.Light` _hud) "Collapsed")))))

(fn `SetCurrentSpell`
  (params (`Spell Type` :type "/Game/Blueprints/Utilities/Enums/ESpellType Enum" :default "NewEnumerator0"))
  (bind _hud (`/Game/Blueprints/Characters/BP_Player.HUD` (`self.Player`)))
  (set `self.Alternative Spell Use` false)
  (set `self.WasActivated` false)
  (`self.CastSpell` (`self.CurrentSpell`))
  (bind _output_get (set `self.CurrentSpell` (`local.Spell Type`)))
  (switch `/Game/Blueprints/Utilities/Enums/ESpellType` _output_get
    (:`NewEnumerator0`
      (`Widget.SetVisibility` (`/Game/Widgets/WBP_HUD.Telekinesis` _hud) "Visible"))
    (:`NewEnumerator3`
      (`Widget.SetVisibility` (`/Game/Widgets/WBP_HUD.Light` _hud) "Visible"))))

(fn `UserConstructionScript`)