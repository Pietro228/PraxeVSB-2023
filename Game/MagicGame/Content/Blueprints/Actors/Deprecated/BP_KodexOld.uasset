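; BP_KodexOld is a spellbook actor, filed as deprecated, that lets the player pick and cast a spell for the wand.
; A timeline and open/close animations toggle the book, switching input mode and walk speed.
; Two page widgets reference the Kodex; SelectSpell starts WBP_SpellCaster, whose pre-cast success updates wand and HUD, then toggles the book.
; While open, Tick deprojects the mouse to position a Niagara cursor.
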(event `self.ReceiveBeginPlay`
  ;[1 0.5625 0] Begin play
  (bind _returnvalue (`NiagaraFunctionLibrary.SpawnSystemAtLocation` "/Game/Niagara/NPS_Cursor.NPS_Cursor"))
  (set `self.FancyCursorParticle` _returnvalue)
  (bind _asbp_player (cast `/Game/Blueprints/Characters/BP_Player` (`GameplayStatics.GetPlayerCharacter` 0)))
  (set `self.Player` _asbp_player)
  (`SceneComponent.SetVisibility` (`self.Book`) false true)
  (bind _returnvalue_2 (`|CreateWidget` "/Game/Widgets/WBP_SpellCaster.WBP_SpellCaster_C"))
  (bind _output_get (set `self.SpellCaster` _returnvalue_2))
  (`UserWidget.AddToViewport` _output_get 10)
  (`Widget.SetVisibility` _output_get "Collapsed")
  (message `/Game/Blueprints/Interfaces/InitializableObjectInterface.InitializeWithReference` (`WidgetComponent.GetWidget` (`self.Page1`)) self)
  (message `/Game/Blueprints/Interfaces/InitializableObjectInterface.InitializeWithReference` (`WidgetComponent.GetWidget` (`self.Page2`)) self)
  (add `/Game/Widgets/WBP_SpellCaster.OnSpellPreCastedSuccessEvent` (`self.SpellCaster`) (delegate `OnSpellCasted`)))

(event `self.ReceiveTick`
  (params (DeltaSeconds :type "Float (single-precision)"))
  (bind _showspecialcursor (`self.ShowSpecialCursor`))
  (`SceneComponent.SetVisibility` (`self.FancyCursorParticle`) _showspecialcursor false)
  (if _showspecialcursor
    (bind (_success _x _y) (`LowEntryExtendedStandardLibrary.GetWindowPosition`))
    (bind _returnvalue (`WidgetLayoutLibrary.GetMousePositionOnPlatform`))
    (bind (_worldposition _worlddirection) (`GameplayStatics.DeprojectScreenToWorld` (`GameplayStatics.GetPlayerController` 0) (`KismetMathLibrary.MakeVector2D` (- (`KismetMathLibrary.BreakVector2D` _returnvalue) _x) (- (`.Y` (`KismetMathLibrary.BreakVector2D` _returnvalue)) _y))))
    (`SceneComponent.K2_SetWorldLocation` (`self.FancyCursorParticle`) (+ _worldposition (* _worlddirection 1.1)) false false)))

(event `OnSpellCasted`
  (params (CastedSpell :type "/Game/Blueprints/Utilities/Enums/ESpellType Enum" :default "NewEnumerator0"))
  ;[0.7813 0 1] OnSpellCasted
  (`/Game/Blueprints/Actors/BP_Wand.SetCurrentSpell` (`self.BP_Wand`) CastedSpell)
  (`Widget.SetVisibility` (`self.SpellCaster`) "Collapsed")
  (`self.Show Hide Kodex`)
  (`/Game/Widgets/WBP_HUD.SetCurrentSpell` (`/Game/Blueprints/Characters/BP_Player.HUD` (`self.Player`)) (`self.SelectedSpell`)))

(event `ShowHideKodexAnimation`
  (bind _returnvalue (`GameplayStatics.GetPlayerController` 0))
  (bind _returnvalue_2 (`GameplayStatics.GetPlayerController` 0))
  (bind _book (`self.Book`))
  ;[1 0.2578 0] Show Hide Kodex
  (bind _output_get (set `self.KodexVisible` (not (`self.KodexVisible`))))
  (if _output_get
    (`SceneComponent.SetVisibility` (`self.Book`) true true)
    (`SkeletalMeshComponent.PlayAnimation` _book "/Game/Models/ViewModel/Book_Anim_BookArmature_Open.Book_Anim_BookArmature_Open" false)
    (bind (_direction _alpha) (`Timeline|MoveKodexTimeline` :!via `PlayFromStart` :!label _label)
      (:`Update`
        (`SceneComponent.K2_SetRelativeLocation` (`self.Book`) (`KismetMathLibrary.MakeVector` 0.0 0.0 (`KismetMathLibrary.Lerp` -200.0 0.0 _alpha)) false false))
      (:`Finished`
        (if (not (`self.KodexVisible`))
          (`SceneComponent.SetVisibility` (`self.Book`) false true)
          (else
            (set `PlayerController.bShowMouseCursor` (`LowEntryExtendedStandardLibrary.WithEditor`) _returnvalue_2)
            (`WidgetBlueprintLibrary.SetInputMode_GameAndUIEx` _returnvalue_2 (`self.SpellCaster`) "LockAlways" true true)
            (set `CharacterMovementComponent.MaxWalkSpeed` 0.0 (`Character.CharacterMovement` (`self.Player`)))
            (set `self.ShowSpecialCursor` true)
            (`LowEntryExtendedStandardLibrary.SetMousePositionInPercentages` 0.2 0.7)))))
    (else
      (set `PlayerController.bShowMouseCursor` false _returnvalue)
      (`WidgetBlueprintLibrary.SetInputMode_GameOnly` _returnvalue)
      (`Widget.SetVisibility` (`self.SpellCaster`) "Collapsed")
      (set `self.ShowSpecialCursor` false)
      (`SkeletalMeshComponent.PlayAnimation` _book "/Game/Models/ViewModel/Book_Anim_BookArmature_Close.Book_Anim_BookArmature_Close" false)
      (set `CharacterMovementComponent.MaxWalkSpeed` 600.0 (`Character.CharacterMovement` (`self.Player`)))
      (goto _label :!via `ReverseFromEnd`))))

(fn `Initialize`
  (params (BP_Wand :type "/Game/Blueprints/Actors/BP_Wand Object Reference"))
  (set `self.BP_Wand` BP_Wand))

(fn `SelectSpell`
  (params (SpellType :type "/Game/Blueprints/Utilities/Enums/ESpellType Enum" :default "NewEnumerator0"))
  (bind _spellcaster (`self.SpellCaster`))
  (set `self.SelectedSpell` SpellType)
  (`Widget.SetVisibility` _spellcaster "Visible")
  (`/Game/Widgets/WBP_SpellCaster.StartCastingSpell` _spellcaster SpellType))

(fn `Show Hide Kodex`
  (`self.ShowHideKodexAnimation`))

(fn `UserConstructionScript`)