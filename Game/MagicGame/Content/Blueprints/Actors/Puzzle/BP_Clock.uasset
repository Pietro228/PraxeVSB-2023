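; Clock puzzle actor that the player solves by turning the minute and hour hands to a fixed target position.
; Interacting with a hand toggles its follow mode, in which Tick traces from the player camera and eases that hand's yaw toward the hit point.
; Yaw rounds to 30-degree steps, feeding index parameters on the Znaky materials and the solution check.
; Solving sets PuzzleCompleted, triggers BPActionComponent once and calls UseSpell(false) on an activated wand.
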(event `self.ReceiveBeginPlay`
  (bind _asbp_player (cast `/Game/Blueprints/Characters/BP_Player` (`GameplayStatics.GetPlayerCharacter` 0)))
  (set `self.Player` _asbp_player))

(event `/Game/Blueprints/Interfaces/InteractableActorInterface.Interacted`
  (params (Hit :type "HitResult Structure"))
  (bind (_bblockinghit _binitialoverlap _time _distance _location _impactpoint _normal _impactnormal _physmat _hitactor _hitcomponent) (`GameplayStatics.BreakHitResult` Hit))
  ;[0 1 0.2031] Event interacted
  (if (== (`self.MinuteHand`) _hitcomponent)
    (bind _output_get (set `self.UsingMinuteHand` (not (stale _output_get))))
    (elif (== _hitcomponent (`self.HourHand`))
      (bind _output_get_2 (set `self.UsingHourHand` (not (stale _output_get_2))))
      (else
        (set `self.UsingMinuteHand` false :!label _label)
        (set `self.UsingHourHand` false)))))

(event `StopFollowingWand`
  ;[0 1 0.2031] Event interacted
  (goto _label))

(event `self.ReceiveTick`
  (params (DeltaSeconds :type "Float (single-precision)"))
  (bind _returnvalue (`self.K2_GetActorLocation`))
  (bind _returnvalue_2 (`GameplayStatics.GetWorldDeltaSeconds`))
  (bind _minutehand (`self.MinuteHand`))
  (bind _hourhand (`self.HourHand`))
  (bind (_returnvalue_roll _returnvalue_pitch _returnvalue_yaw) (`KismetMathLibrary.BreakRotator` (`SceneComponent.K2_GetComponentRotation` _hourhand)))
  (bind (_returnvalue_roll_2 _returnvalue_pitch_2 _returnvalue_yaw_2) (`KismetMathLibrary.BreakRotator` (`SceneComponent.K2_GetComponentRotation` _minutehand)))
  (bind _wand (`/Game/Blueprints/Characters/BP_Player.Wand` (`self.Player`)))
  (bind _firstpersoncamera (`/Game/Blueprints/Characters/BP_Player.FirstPersonCamera` (`self.Player`)))
  (bind _returnvalue_3 (`SceneComponent.K2_GetComponentLocation` _firstpersoncamera))
  (bind _returnvalue_4 (+ _returnvalue_yaw 180.0))
  (bind _returnvalue_5 (mod (select `bool` (< _returnvalue_yaw_2 0.0) :`false` _returnvalue_yaw_2 :`true` (+ _returnvalue_yaw_2 360.0) :!type "Float (double-precision)") 360.0))
  (bind _returnvalue_6 (`KismetMathLibrary.MapRangeClamped` (- (`KismetMathLibrary.Conv_IntToDouble` (`KismetMathLibrary.Round` (/ _returnvalue_4 30.0))) 1.0) 0.0 11.0 11.0))
  (bind _returnvalue_7 (`KismetMathLibrary.MapRangeClamped` (+ (`KismetMathLibrary.Conv_IntToDouble` (`KismetMathLibrary.Round` (/ _returnvalue_5 30.0))) -1.0) 0.0 11.0 11.0))
  (if (not (and (== _returnvalue_7 11.0) (== _returnvalue_6 4.0)))
    (if (or (`self.UsingMinuteHand`) (`self.UsingHourHand`))
      (bind _outhit (`KismetSystemLibrary.LineTraceSingle` :`Start` _returnvalue_3 :`End` (+ _returnvalue_3 (* (`SceneComponent.GetForwardVector` _firstpersoncamera) 2000)) :`TraceChannel` "TraceTypeQuery1" :`bTraceComplex` true :`DrawDebugType` "ForDuration" :`bIgnoreSelf` false))
      (bind (_bblockinghit _binitialoverlap _time _distance _location) (`GameplayStatics.BreakHitResult` _outhit))
      (if _bblockinghit
        (if (`self.UsingMinuteHand`)
          (bind (_returnvalue_roll_3 _returnvalue_pitch_3 _returnvalue_yaw_3) (`KismetMathLibrary.BreakRotator` (`KismetMathLibrary.FindLookAtRotation` _returnvalue _location)))
          (`SceneComponent.K2_SetRelativeRotation` _minutehand (`KismetMathLibrary.RInterpTo` (`SceneComponent.RelativeRotation` _minutehand) (`KismetMathLibrary.MakeRotator` 0.0 0.0 (+ _returnvalue_yaw_3 90.0)) _returnvalue_2 1.0) false false)
          (`KismetSystemLibrary.PrintString` (`KismetStringLibrary.Conv_DoubleToString` (mod _returnvalue_5 30.0)))
          (`MeshComponent.SetScalarParameterValueOnMaterials` (`self.Znaky`) "MinuteHandIndex" _returnvalue_7)
          (elif (`self.UsingHourHand`)
            (bind (_returnvalue_roll_4 _returnvalue_pitch_4 _returnvalue_yaw_4) (`KismetMathLibrary.BreakRotator` (`KismetMathLibrary.FindLookAtRotation` _returnvalue _location)))
            (`SceneComponent.K2_SetRelativeRotation` _hourhand (`KismetMathLibrary.RInterpTo` (`SceneComponent.RelativeRotation` _hourhand) (`KismetMathLibrary.MakeRotator` 0.0 0.0 (- _returnvalue_yaw_4 90.0)) _returnvalue_2 1.0) false false)
            (`KismetSystemLibrary.PrintString` (`KismetStringLibrary.Conv_DoubleToString` _returnvalue_4))
            (`MeshComponent.SetScalarParameterValueOnMaterials` (`self.Znaky`) "HourHandIndex" _returnvalue_6)))))
    (else
      (`KismetSystemLibrary.PrintString` "Hands are in the right position!")
      (`/Engine/EditorBlueprintResources/StandardMacros.DoOnce` false
        (:`Completed`
          (set `self.PuzzleCompleted` true)
          (`/Game/Blueprints/Components/BP_ActionComponent.Trigger` (`self.BP_ActionComponent`))
          (if (`/Game/Blueprints/Actors/BP_Wand.WasActivated` _wand)
            (`/Game/Blueprints/Actors/BP_Wand.UseSpell` _wand false)))))))

(fn `UserConstructionScript`)