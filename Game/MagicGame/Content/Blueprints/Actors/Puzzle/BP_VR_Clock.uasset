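; BP_VR_Clock is a puzzle clock with two physics-driven hands that signals when both reach their target angles.
; RelocateHand converts a hit location into a signed yaw, measured against the Hour constraint's right vector, and sets it as the chosen hand constraint's angular orientation target.
; A delayed Tick keeps the hands awake and fires OnClockAligned once when both yaws sit within a small tolerance of the desired angles.
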(event `self.ReceiveTick`
  (params (DeltaSeconds :type "Float (single-precision)"))
  (bind _desiredhourandgle (`self.DesiredHourAndgle`))
  (bind _desiregminuteangle (`self.DesiregMinuteAngle`))
  (bind (_returnvalue_roll _returnvalue_pitch _returnvalue_yaw) (`KismetMathLibrary.BreakRotator` (`SceneComponent.K2_GetComponentRotation` (`self.HourHand`))))
  (bind (_returnvalue_roll_2 _returnvalue_pitch_2 _returnvalue_yaw_2) (`KismetMathLibrary.BreakRotator` (`SceneComponent.K2_GetComponentRotation` (`self.MinuteHand`))))
  (bind _returnvalue (mod _returnvalue_yaw_2 360.0))
  (bind _returnvalue_2 (mod (+ _returnvalue_yaw 180.0) 360.0))
  (`KismetSystemLibrary.Delay` 0.1)
  (`PrimitiveComponent.WakeAllRigidBodies` (`self.HourHand`))
  (`PrimitiveComponent.WakeAllRigidBodies` (`self.MinuteHand`))
  (if (and (and (> _returnvalue (- _desiregminuteangle 5.0)) (< _returnvalue (+ _desiregminuteangle 5.0))) (and (> _returnvalue_2 (- _desiredhourandgle 5.0)) (< _returnvalue_2 (+ _desiredhourandgle 5.0))))
    (`/Engine/EditorBlueprintResources/StandardMacros.DoOnce` false
      (:`Completed`
        (`self.OnClockAligned`)))))

(event `self.ReceiveBeginPlay`)

(event `RelocateHand`
  (params (HitLoc :type "Vector Structure") (bHitHour :type Boolean))
  (bind _hour (`self.hour`))
  (bind _x (.x (- HitLoc (`SceneComponent.K2_GetComponentLocation` (`self.Clock`)))))
  (bind _returnvalue (`KismetMathLibrary.DegAcos` (`KismetMathLibrary.Dot_VectorVector` (`KismetMathLibrary.Normal` (`KismetMathLibrary.MakeVector` _x (.y (- HitLoc (`SceneComponent.K2_GetComponentLocation` (`self.Clock`)))))) (`SceneComponent.GetRightVector` _hour))))
  (`PhysicsConstraintComponent.SetAngularOrientationTarget` (select `bool` bHitHour :`false` (`self.Minute`) :`true` _hour) (`KismetMathLibrary.MakeRotator` 0.0 0.0 (`KismetMathLibrary.SelectFloat` (* _returnvalue -1.0) _returnvalue (< _x 0.0)))))

(fn `UserConstructionScript`)