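; BP_MS_Fire is a magic-spell Blueprint, named for fire, built from four child-actor spell blocks.
; On BeginPlay it runs the parent logic, then casts each child actor to BP_MagicSpellBlock and gathers them in AllSpellBlocks.
; A failed cast stops the gathering.
; It adds no other behavior: overlap and tick events are disabled, and the construction script only calls the parent.
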(event `self.ReceiveBeginPlay`
  (`parent.ReceiveBeginPlay`)
  (for _array_element (`|MakeArray` (`self.BP_MagicSpellBlock`) (`self.BP_MagicSpellBlock1`) (`self.BP_MagicSpellBlock2`) (`self.BP_MagicSpellBlock3`))
    (bind _asbp_magic_spell_block (cast `/Game/FoxyPersonalTesting/BP_MagicSpellBlock` (`ChildActorComponent.ChildActor` _array_element)))
    (`KismetArrayLibrary.Array_Add` (`self.AllSpellBlocks`) _asbp_magic_spell_block)))

(fn `UserConstructionScript`
  (`parent.UserConstructionScript`))