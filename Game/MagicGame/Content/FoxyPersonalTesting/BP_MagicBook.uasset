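; Grabbable VR spellbook (Kodex) where the player picks spells to charge the wand held in the right hand.
; Show-Kodex input or left trigger drives the open/close animation, with input mode and mappings switching for UI use.
; Two page widgets receive book references and spell unlocks.
; Selecting a spell closes the book and spawns its BP_MS drawing actor before the camera; success callbacks charge the wand.
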(event `self.ReceiveBeginPlay`
  (bind _returnvalue (`GameplayStatics.GetPlayerController` 0))
  (`/Game/Blueprints/Utilities/BlueprintUtilities/BPFL_qol.ToggleInputMappings` _returnvalue "NewEnumerator2" true)
  (`self.InitializeComponentsAndVariables` null)
  (`EnhancedInputSubsystemInterface.AddMappingContext` (pcsubsystem `EnhancedInputLocalPlayerSubsystem` _returnvalue) "/Game/VRTemplate/Input/IMC_VR_Kodex.IMC_VR_Kodex" 0 (struct)))

(event `OpenKodex`
  ;[0.1562 0.05195 0] Open or close kodex by events
  (set `/Game/FoxyPersonalTesting/ABP_MagicBook.bOpenAnim` true (`self.MagicBookABP`))
  (set `self.bIsMagicBookOpen` true))

(event `EnhancedInput|/Game/Input/Actions/IA_ShowKodex`
  (params (ActionValue :type Boolean) (ElapsedSeconds :type "Float (double-precision)") (TriggeredSeconds :type "Float (double-precision)") (InputAction :type "InputAction Object Reference" :default "/Game/Input/Actions/IA_ShowKodex.IA_ShowKodex"))
  ;[0.99 1 1] Input handling
  (:`Started`
    (if (not (`self.bIsMagicBookOpen`)) :!label _label
      (`self.OpenKodex`)
      (else
        (`self.CloseKodex`)))))

(event `CloseKodex`
  (bind _returnvalue (`GameplayStatics.GetPlayerController` 0))
  ;[0.1562 0.05195 0] Open or close kodex by events
  (set `/Game/FoxyPersonalTesting/ABP_MagicBook.bOpenAnim` false (`self.MagicBookABP`))
  (`/Game/Blueprints/Utilities/BlueprintUtilities/BPFL_qol.ToggleInputMappings` _returnvalue "NewEnumerator0" true)
  (set `PlayerController.bShowMouseCursor` false _returnvalue)
  (`WidgetBlueprintLibrary.SetInputMode_GameOnly` _returnvalue)
  (set `self.bIsMagicBookOpen` false))

(event `/Game/FoxyPersonalTesting/VR_Input.OnLeftTrigger`
  (goto _label))

(event `/Game/FoxyPersonalTesting/Vr_to_actors.OnGrab`
  (params (Player :type "/Game/Blueprints/Characters/BP_VRPL Object Reference"))
  (bind _output_get (set `self.Player` Player))
  (bind _heldcomponentright (`/Game/Blueprints/Characters/BP_VRPL.HeldComponentRight` _output_get))
  (`/Engine/EditorBlueprintResources/StandardMacros.IsValid` _heldcomponentright
    (:`Is Valid`
      (bind _asbp_wand_changed (cast `/Game/FoxyPersonalTesting/BP_Wand_Changed` (`ActorComponent.GetOwner` _heldcomponentright)))
      (set `self.Wand` _asbp_wand_changed))))

(event `PreCastSuccessfulEvent`
  (params (CastedSpell :type "/Game/Blueprints/Utilities/Enums/ESpellType Enum" :default "NewEnumerator0"))
  ;[0 0.005208 0.005122] Called when selected spell was drawn successfully
  (`self.CloseKodex`)
  (`/Game/FoxyPersonalTesting/BP_Wand_Changed.SetAndChargeWand` (`self.Wand`) true CastedSpell)
  (set `self.bIsMagicBookOpen` false)
  (`/Game/Widgets/WBP_HUD.SetCurrentSpell` (`self.HUD`) CastedSpell))

(event `/Game/FoxyPersonalTesting/Vr_to_actors.OnDrop`
  (set `self.Player` null)
  (set `self.Wand` null)
  (`self.CloseKodex`))

(event `/Game/FoxyPersonalTesting/Vr_to_actors.OnDropAlt`
  (set `self.Wand` null))

(event `/Game/Blueprints/Interfaces/KodexPageInterface.UnlockSpell`
  (params (`Spell Type` :type "/Game/Blueprints/Utilities/Enums/ESpellType Enum" :default "NewEnumerator0"))
  (message `/Game/Blueprints/Interfaces/KodexPageInterface.UnlockSpell` (`WidgetComponent.GetWidget` (`self.PageLeft`)) `Spell Type`)
  (message `/Game/Blueprints/Interfaces/KodexPageInterface.UnlockSpell` (`WidgetComponent.GetWidget` (`self.PageRight`)) `Spell Type`))

(event `BookOpened`
  (bind _returnvalue (`GameplayStatics.GetPlayerController` 0))
  ;[0.3229 0.3229 0.3229] Called when books get opened (animation of opening ends)
  (`/Game/Blueprints/Utilities/BlueprintUtilities/BPFL_qol.ToggleInputMappings` _returnvalue)
  (set `PlayerController.bShowMouseCursor` true _returnvalue)
  (`WidgetBlueprintLibrary.SetInputMode_GameAndUIEx` _returnvalue null "LockAlways" false true))

(event `self.OnCastSucces`
  (params (Spelltype :type "/Game/Blueprints/Utilities/Enums/ESpellType Enum" :default "NewEnumerator0"))
  (`/Game/FoxyPersonalTesting/BP_Wand_Changed.SetAndChargeWand` (`self.Wand`) true Spelltype)
  (set `self.bIsCasting` false))

(fn `GetMagicStoneType`
  (returns (NewParam :type "/Game/Blueprints/Utilities/Enums/ESpellType Enum"))
  (return "NewEnumerator0"))

(fn `InitializeComponentsAndVariables`
  (params (Wand :type "/Game/FoxyPersonalTesting/BP_Wand_Changed Object Reference"))
  (`|ExecutionSequence`
    (:`then_0`
      ;[0 0 0] Initializes pages (widgets)
      (message `/Game/Blueprints/Interfaces/VR_PageInterface.InitializePageVR` (`WidgetComponent.GetWidget` (`self.PageRight`)) self)
      (message `/Game/Blueprints/Interfaces/VR_PageInterface.InitializePageVR` (`WidgetComponent.GetWidget` (`self.PageLeft`)) self))
    (:`then_1`
      ;[0 1 0.9834] Set reference variables (anim instance, wand)
      (set `self.Wand` Wand)
      (bind _asabp_magic_book (cast `/Game/FoxyPersonalTesting/ABP_MagicBook` (`SkeletalMeshComponent.GetAnimInstance` (`self.Kodex`))))
      (set `self.MagicBookABP` _asabp_magic_book))
    (:`then_2`
      ;[1 0.03955 0.03955] Bind events
      (add `/Game/FoxyPersonalTesting/ABP_MagicBook.BookOpenedDispatcher` (`self.MagicBookABP`) (`|CreateDelegate` :!event `BookOpened`)))))

(fn `PreCastSpell`
  (params (SpellType :type "/Game/Blueprints/Utilities/Enums/ESpellType Enum" :default "NewEnumerator0"))
  (bind _player (`self.Player`))
  (bind _returnvalue (`KismetMathLibrary.MakeRotator` 0.0 0.0 (.yaw (.rotation (`SceneComponent.K2_GetComponentToWorld` (`/Game/Blueprints/Characters/BP_VRPL.Camera` _player))))))
  (`/Engine/EditorBlueprintResources/StandardMacros.IsValid` (`self.Wand`)
    (:`Is Valid`
      (if (not (`self.bIsCasting`))
        (set `self.SelectedSpell` SpellType)
        (`self.CloseKodex`)
        ;[0.3958 0.3958 0] Comment
        (`/Engine/EditorBlueprintResources/StandardMacros.IsValid` _player
          (:`Is Valid`
            (`/Game/FoxyPersonalTesting/BP_Wand_Changed.CastSpell` :`self` (`self.Wand`))
            (bind _returnvalue_2 (`|SpawnActorFromClass` (select `/Game/Blueprints/Utilities/Enums/ESpellType` SpellType :`NewEnumerator0` "/Game/FoxyPersonalTesting/MagicSpells/BP_MS_Telekinesis.BP_MS_Telekinesis_C" :`NewEnumerator3` "/Game/FoxyPersonalTesting/MagicSpells/BP_MS_Light.BP_MS_Light_C" :`NewEnumerator1` "/Game/FoxyPersonalTesting/MagicSpells/BP_MS_Fire.BP_MS_Fire_C" :`NewEnumerator2` "/Game/FoxyPersonalTesting/MagicSpells/BP_MS_Freeze.BP_MS_Freeze_C" :`NewEnumerator5` "/Game/FoxyPersonalTesting/MagicSpells/BP_MS_Bread.BP_MS_Bread_C" :!type "Actor Class Reference") (`KismetMathLibrary.MakeTransform` (+ (.location (`SceneComponent.K2_GetComponentToWorld` (`/Game/Blueprints/Characters/BP_VRPL.Camera` _player))) (`KismetMathLibrary.GreaterGreater_VectorRotator` (100.0 0.0 0.0) _returnvalue))) "AdjustIfPossibleButDontSpawnIfColliding" "OverrideRootScale" null null))
            (`/Engine/EditorBlueprintResources/StandardMacros.IsValid` _returnvalue_2
              (:`Is Valid`
                (message `/Game/FoxyPersonalTesting/MagicSpells/I_MagicSpell.OnSpawn` _returnvalue_2 self _returnvalue (`self.SelectedSpell`))
                (set `self.bIsCasting` true)))))))))

(fn `UserConstructionScript`)