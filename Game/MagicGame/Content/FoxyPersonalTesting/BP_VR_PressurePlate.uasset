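; BP_VR_PressurePlate is a pressure plate that calls OnActivated when actors enter its box and OnDisabled when the last one leaves.
; An overlap counter and a DoOnce, reset at zero, keep activation to one call per occupied period.
; Two Niagara effects switch trail color on every begin or end overlap, even if other actors remain.
; Tick steadily yaws the particle handle.
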(event `self.ReceiveBeginPlay`)

(event `self.Box.OnComponentBeginOverlap`
  (params (OverlappedComponent :type "PrimitiveComponent Object Reference") (OtherActor :type "Actor Object Reference") (OtherComp :type "PrimitiveComponent Object Reference") (OtherBodyIndex :type Integer) (bFromSweep :type Boolean) (SweepResult :type "HitResult Structure (by ref)"))
  (bind _returnvalue (`KismetMathLibrary.Conv_ColorToLinearColor` (`|GetArrayItem` (`self.Colors`) 1)))
  (`/Engine/EditorBlueprintResources/StandardMacros.IncrementInt` (`self.OverlappingActors`)
    (:`  `
      (`FXSystemComponent.SetColorParameter` (`self.NS_PressurePlate`) "user.TrailColor" _returnvalue)
      (`FXSystemComponent.SetColorParameter` (`self.NS_PressurePlate1`) "user.TrailColor" _returnvalue)
      (`/Engine/EditorBlueprintResources/StandardMacros.DoOnce` false :!label _label
        (:`Completed`
          (`self.OnActivated`))))))

(event `self.Box.OnComponentEndOverlap`
  (params (OverlappedComponent :type "PrimitiveComponent Object Reference") (OtherActor :type "Actor Object Reference") (OtherComp :type "PrimitiveComponent Object Reference") (OtherBodyIndex :type Integer))
  (bind _returnvalue (`KismetMathLibrary.Conv_ColorToLinearColor` (`|GetArrayItem` (`self.Colors`))))
  (`/Engine/EditorBlueprintResources/StandardMacros.DecrementInt` (`self.OverlappingActors`)
    (:`  `
      (`FXSystemComponent.SetColorParameter` (`self.NS_PressurePlate`) "user.TrailColor" _returnvalue)
      (`FXSystemComponent.SetColorParameter` (`self.NS_PressurePlate1`) "user.TrailColor" _returnvalue)
      (if (== (`self.OverlappingActors`) 0)
        (`self.OnDisabled`)
        (goto _label :!via `Reset`)))))

(event `self.ReceiveTick`
  (params (DeltaSeconds :type "Float (single-precision)"))
  (`SceneComponent.K2_AddRelativeRotation` (`self.ParticlesHandle`) (`KismetMathLibrary.MakeRotator` 0.0 0.0 (* DeltaSeconds 20.0)) false false))

(fn `UserConstructionScript`)