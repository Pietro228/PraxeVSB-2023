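; Wand actor that casts the selected spell from a camera raycast, with each use input toggling it on or off.
; Telekinesis flies a physics object to the grab point via timeline and PhysicsHandle, holds it until timeout or toggle-off, optionally launching it forward.
; Light fades a point light and recolours wand-tip particles; Fire messages the hit actor to ignite.
; Freeze is an empty stub.
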(event `self.ReceiveTick`
  (params (DeltaSeconds :type "Float (single-precision)"))
  ;[1 0.9015 0] Tick
  (switch `/Game/Blueprints/Utilities/Enums/ESpellType` (`self.CurrentSpell`)
    (:`NewEnumerator0`
      (`PhysicsHandleComponent.SetTargetLocation` (`self.PhysicsHandle`) (`SceneComponent.K2_GetComponentLocation` (`self.GrabLocation`))))))

(event `EnhancedInput|/Game/Input/Actions/IA_UseWand`
  (params (ActionValue :type Boolean) (ElapsedSeconds :type "Float (double-precision)") (TriggeredSeconds :type "Float (double-precision)") (InputAction :type "InputAction Object Reference" :default "/Game/Input/Actions/IA_UseWand.IA_UseWand"))
  (:`Started`
    (bind _output_get (set `self.bIsSpellActive` (not (stale _output_get))))
    (bind _hit (`/Game/Blueprints/Utilities/BlueprintUtilities/BPFL_qol.Raycast` (`self.Camera`) 1000.0 "Persistent"))
    (`self.CastSpell` _hit _output_get)))

(event `SpellTelekinesis`
  (params (Hit :type "HitResult Structure") (`Act_/_DeAact` :type Boolean))
  (bind (_bblockinghit _binitialoverlap _time _distance _location _impactpoint _normal _impactnormal _physmat _hitactor _hitcomponent) (`GameplayStatics.BreakHitResult` Hit))
  ;[0.6406 0 1] Telekinesis Grab
  (if `Act_/_DeAact`
    (if _bblockinghit
      (if (`SceneComponent.IsSimulatingPhysics` _hitcomponent "None")
        (bind _output_get (set `self.SpellTelekinesisHit Component` _hitcomponent))
        (`PhysicsHandleComponent.GrabComponentAtLocation` (`self.PhysicsHandle`) _output_get "None" _location)
        (bind (_direction _location_2) (`Timeline|FliToWand` :!via `PlayFromStart`)
          (:`Update`
            (`PhysicsHandleComponent.SetTargetLocation` (`self.PhysicsHandle`) (`KismetMathLibrary.VLerp` _location (`SceneComponent.K2_GetComponentLocation` (`self.GrabLocation`)) _location_2)))
          (:`Finished`
            (set `self.TelekinesisActive` true)
            (`Timeline|StopTelekinesisTimeline` :!via `PlayFromStart`
              (:`Finished`
                (set `self.TelekinesisActive` false :!label _label)
                (`PhysicsHandleComponent.ReleaseComponent` (`self.PhysicsHandle`))
                (if (`self.Alternative Spell Use`)
                  (`PrimitiveComponent.AddImpulse` (`self.SpellTelekinesisHit Component`) (* (`SceneComponent.GetForwardVector` (`self.Camera`)) 1000) "None" true))))))))
    (else
      (`TimelineComponent.Stop` (`self.StopTelekinesisTimeline`))
      (goto _label))))

(event `SpellLight`
  (params (Hit :type "HitResult Structure") (`Act_/_DeAact` :type Boolean))
  ;[0 0.4375 1] Light Spell
  (`self.SetAndChargeWand` `Act_/_DeAact` "NewEnumerator3")
  (if `Act_/_DeAact`
    (bind (_direction _alpha) (`Timeline|SpellLightIntesityTimeline` :!label _label_2)
      (:`Update`
        (`LightComponent.SetIntensity` (`self.PointLight`) (`KismetMathLibrary.Lerp` 0.0 3000.0 _alpha))))
    (else
      (goto _label_2 :!via `Reverse`))))

(event `SpellFire`
  (params (Hit :type "HitResult Structure"))
  (bind (_bblockinghit _binitialoverlap _time _distance _location _impactpoint _normal _impactnormal _physmat _hitactor) (`GameplayStatics.BreakHitResult` Hit))
  (if _bblockinghit
    (message `/Game/Blueprints/Interfaces/SpellReactionInterface.LightOnFire` _hitactor)))

(event `SpellFreeze`
  (params (Hit :type "HitResult Structure")))

(fn `CastSpell`
  (params (HitObject :type "HitResult Structure") (`bAct_/_DeAct` :type Boolean))
  (switch `/Game/Blueprints/Utilities/Enums/ESpellType` (`self.CurrentSpell`)
    (:`NewEnumerator0`
      (`self.SpellTelekinesis` HitObject `bAct_/_DeAct`))
    (:`NewEnumerator3`
      (`self.SpellLight` HitObject `bAct_/_DeAct`))
    (:`NewEnumerator1`
      (`self.SpellFire` HitObject))
    (:`NewEnumerator2`
      (`self.SpellFreeze` HitObject))))

(fn `Initialize`
  (params (Player :type "/Game/FoxyPersonalTesting/BP_PL Object Reference") (Camera :type "SceneComponent Object Reference"))
  (set `self.Player` Player)
  (set `self.Camera` Camera)
  (return))

(fn `SetAndChargeWand`
  (params (bCharge :type Boolean) (SpellType :type "/Game/Blueprints/Utilities/Enums/ESpellType Enum" :default "NewEnumerator0"))
  (locals (BaseSpawnRate :type "Float (double-precision)" :default 1000.0))
  (bind _wandtip (`self.WandTip`))
  (set `self.CurrentSpell` SpellType)
  (`NiagaraComponent.SetVariableFloat` _wandtip "user.SpawnRate" (`KismetMathLibrary.SelectFloat` (`local.BaseSpawnRate`) 0.0 bCharge))
  (`NiagaraComponent.SetVariableLinearColor` _wandtip "user.ChargeColor" (`|GetArrayItem` (`self.SpellCollors`) (`KismetMathLibrary.Conv_ByteToInt` SpellType))))

(fn `UserConstructionScript`)