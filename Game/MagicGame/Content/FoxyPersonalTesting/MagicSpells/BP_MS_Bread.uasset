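; Bread variant of a magic spell, built as a child Blueprint that supplies a bread-shaped vertex set.
; CreateSpell reads the vertices of the Bread static mesh's first section at LOD 0 into Verticies, then calls the parent CreateSpell.
; CreateSpellEvent triggers that function, while the construction script and active lifecycle events only forward to the parent.
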(event `self.ReceiveBeginPlay`
  (`parent.ReceiveBeginPlay`))

(event `self.ReceiveTick`
  (params (DeltaSeconds :type "Float (single-precision)"))
  (`parent.ReceiveTick` DeltaSeconds))

(event `self.CreateSpellEvent`
  (`self.CreateSpell`))

(fn `CreateSpell`
  (bind _vertices (`KismetProceduralMeshLibrary.GetSectionFromStaticMesh` "/Game/FoxyPersonalTesting/MagicSpells/bread.bread"))
  (set `self.Verticies` _vertices)
  (`parent.CreateSpell`)
  (return))

(fn `UserConstructionScript`
  (`parent.UserConstructionScript`))