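; BP_MS_Fire is a fire magic spell Blueprint that builds its shape out of BP_MagicSpellBlock actors on BeginPlay.
; It reads the vertices of section 0 of a static mesh and spawns one block per vertex, rotated -90 degrees about X and offset by the root's world location.
; Each block is attached to the spell, keeping its world transform, and stored in AllSpellBlocks.
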(event `self.ReceiveBeginPlay`
  (`parent.ReceiveBeginPlay`)
  ;[0 0.5312 1] Creates spell blocks from desired mesh and attaches them to magic spell (aka the child that will be spawned from this BP)(well currently just here but dont mind that :D)
  (bind _vertices (`KismetProceduralMeshLibrary.GetSectionFromStaticMesh` "/Game/FoxyPersonalTesting/MagicSpells/untitled.untitled"))
  (for _array_element _vertices
    (bind _returnvalue (`|SpawnActorFromClass` "/Game/FoxyPersonalTesting/MagicSpells/BP_MagicSpellBlock.BP_MagicSpellBlock_C" (`KismetMathLibrary.MakeTransform` (+ (`KismetMathLibrary.RotateAngleAxis` _array_element -90.0 (1.0 0.0 0.0)) (`SceneComponent.K2_GetComponentLocation` (`self.DefaultSceneRoot`)))) "Undefined" "OverrideRootScale" null null))
    (`self.K2_AttachToActor` _returnvalue self "None" "KeepWorld" "KeepWorld" "KeepWorld" true)
    (`KismetArrayLibrary.Array_Add` (`self.AllSpellBlocks`) _returnvalue)))

(event `self.ReceiveTick`
  (params (DeltaSeconds :type "Float (single-precision)"))
  (`parent.ReceiveTick` DeltaSeconds))

(fn `UserConstructionScript`
  (`parent.UserConstructionScript`))