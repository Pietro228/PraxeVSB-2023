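; BP_MagicSpell is a spell actor that tracks the spell blocks passed and reports a successful cast to its magic book.
; OnSpawn stores the MagicBook reference, and OnBlockPassed adds each block uniquely to PassedSpellBlocks.
; When the passed count equals AllSpellBlocks, it sends OnCastSuccesMessage with its SpellType, then destroys every block and itself.
; Debug prints remain, and AllSpellBlocks is not populated in these graphs.
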(event `self.ReceiveBeginPlay`)

(event `/Game/FoxyPersonalTesting/MagicSpells/I_MagicSpell.OnBlockPassed`
  (params (SpellBlock :type "/Game/FoxyPersonalTesting/MagicSpells/BP_MagicSpellBlock Object Reference"))
  (bind _passedspellblocks (`self.PassedSpellBlocks`))
  (`KismetSystemLibrary.PrintString` (`KismetSystemLibrary.GetDisplayName` SpellBlock))
  (`KismetArrayLibrary.Array_AddUnique` _passedspellblocks SpellBlock)
  (if (== (`KismetArrayLibrary.Array_Length` (`self.AllSpellBlocks`)) (`KismetArrayLibrary.Array_Length` _passedspellblocks))
    (message `/Game/FoxyPersonalTesting/MagicSpells/I_MagicSpell.OnCastSucces` (stale `/Game/FoxyPersonalTesting/MagicSpells/I_MagicSpell.OnSpawn` MagicBook) (`self.SpellType`))
    (`KismetSystemLibrary.PrintString` "Hello")
    (for _array_element (`self.AllSpellBlocks`)
      (`self.K2_DestroyActor` _array_element))
    (`self.K2_DestroyActor`)))

(event `/Game/FoxyPersonalTesting/MagicSpells/I_MagicSpell.OnSpawn`
  (params (MagicBook :type "Actor Object Reference"))
  (set `self.MagicBook` MagicBook))

(fn `UserConstructionScript`)