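; Wave Function Collapse generator that builds a grid maze of connected wall tiles around a predefined path.
; MakeGrid spawns BP_WFCB cells and a border, then collapses cells along the straight-segment Way route first.
; It repeatedly collapses a random lowest-entropy cell, recursively propagating side-connection constraints to neighbours, and places tiles as rotated mesh instances.
; Overlapping WayTriger once scatters bread instances along the route.
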(event `MakeGrid`
  (bind _uncollapsedcells (`self.UnCollapsedCells`))
  (bind _returnvalue (`KismetArrayLibrary.Array_IsNotEmpty` _uncollapsedcells))
  (`self.Initialize` (`|MakeArray` (`self.ConstructWFCB_Type` "NewEnumerator0" (`|MakeArray` "NewEnumerator0" "NewEnumerator1" "NewEnumerator2" "NewEnumerator3" :!type "/Game/WFC_Gen/EWFCB_Side Enum")) (`self.ConstructWFCB_Type` "NewEnumerator1" (`|MakeArray` "NewEnumerator0" "NewEnumerator3" :!type "/Game/WFC_Gen/EWFCB_Side Enum")) (`self.ConstructWFCB_Type` "NewEnumerator2" (`|MakeArray` "NewEnumerator0" "NewEnumerator1" :!type "/Game/WFC_Gen/EWFCB_Side Enum")) (`self.ConstructWFCB_Type` "NewEnumerator3" (`|MakeArray` "NewEnumerator2" "NewEnumerator3" :!type "/Game/WFC_Gen/EWFCB_Side Enum")) (`self.ConstructWFCB_Type` "NewEnumerator4" (`|MakeArray` "NewEnumerator2" "NewEnumerator1" :!type "/Game/WFC_Gen/EWFCB_Side Enum")) (`self.ConstructWFCB_Type` "NewEnumerator5" (`|MakeArray` "NewEnumerator1" "NewEnumerator3" :!type "/Game/WFC_Gen/EWFCB_Side Enum")) (`self.ConstructWFCB_Type` "NewEnumerator6" (`|MakeArray` "NewEnumerator0" "NewEnumerator2" :!type "/Game/WFC_Gen/EWFCB_Side Enum")) (`self.ConstructWFCB_Type` "NewEnumerator7" (`|MakeArray` "NewEnumerator0" "NewEnumerator2" "NewEnumerator3" :!type "/Game/WFC_Gen/EWFCB_Side Enum")) (`self.ConstructWFCB_Type` "NewEnumerator8" (`|MakeArray` "NewEnumerator0" "NewEnumerator2" "NewEnumerator1" :!type "/Game/WFC_Gen/EWFCB_Side Enum")) (`self.ConstructWFCB_Type` "NewEnumerator9" (`|MakeArray` "NewEnumerator3" "NewEnumerator0" "NewEnumerator1" :!type "/Game/WFC_Gen/EWFCB_Side Enum")) (`self.ConstructWFCB_Type` "NewEnumerator10" (`|MakeArray` "NewEnumerator3" "NewEnumerator2" "NewEnumerator1" :!type "/Game/WFC_Gen/EWFCB_Side Enum")) (`self.ConstructWFCB_Type` "NewEnumerator19" (`|MakeArray`)) (`self.ConstructWFCB_Type` "NewEnumerator20" (`|MakeArray` "NewEnumerator0" :!type "/Game/WFC_Gen/EWFCB_Side Enum")) (`self.ConstructWFCB_Type` "NewEnumerator21" (`|MakeArray` "NewEnumerator1" :!type "/Game/WFC_Gen/EWFCB_Side Enum")) (`self.ConstructWFCB_Type` "NewEnumerator22" (`|MakeArray` "NewEnumerator2" :!type "/Game/WFC_Gen/EWFCB_Side Enum")) (`self.ConstructWFCB_Type` "NewEnumerator23" (`|MakeArray` "NewEnumerator3" :!type "/Game/WFC_Gen/EWFCB_Side Enum"))))
  (bind _waytoconstruct (`self.PreConstructGrid` (`self.Way`)))
  (`self.PreConstructGridUpdate` _waytoconstruct)
  (if _returnvalue :!label _label
    (`KismetSystemLibrary.Delay` 0.0)
    (if _returnvalue
      (bind _collapsedcell (`self.CollapseRandomCell` _uncollapsedcells))
      (if _returnvalue
        (bind (_x _y) (`/Game/WFC_Gen/Blocks/BP_WFCB.GetPosition` _collapsedcell))
        (`self.UpdateGrid` (make `/Game/WFC_Gen/F_Position` _x _y))
        (goto _label)
        (else
          (goto _label)))
      (else
        (goto _label)))))

(event `self.ReceiveTick`
  (params (DeltaSeconds :type "Float (single-precision)")))

(event `self.ReceiveBeginPlay`)

(event `self.WayTriger.OnActorBeginOverlap`
  (params (OverlappedActor :type "Actor Object Reference") (OtherActor :type "Actor Object Reference"))
  (`/Engine/EditorBlueprintResources/StandardMacros.DoOnce` false
    (:`Completed`
      (for (_array_element _array_index) (`self.Grid`)
        (for (_ _array_index_2) (`.Y_Blocks_8_E43C58594D4CAD8B76D849A3CB4CB618` (break `/Game/WFC_Gen/ARR_WFCB_2D` _array_element))
          (if (`KismetArrayLibrary.Array_Contains` (`self.WayToConstruct`) (make `/Game/WFC_Gen/F_Position` _array_index _array_index_2))
            (`InstancedStaticMeshComponent.AddInstance` (`self.WFCB_BreadInstances`) (`KismetMathLibrary.MakeTransform` (`KismetMathLibrary.MakeVector` (`KismetMathLibrary.Conv_IntToDouble` (* _array_index 800)) (`KismetMathLibrary.Conv_IntToDouble` (* _array_index_2 800)) 30.0) (`KismetMathLibrary.MakeRotator` 0.0 0.0 (`KismetMathLibrary.RandomFloatInRange` 0.0 360.0)) (0.5 0.5 0.5)) false)))))))

(fn `CheckAndUpdateCell`
  (params (Pointer :type "/Game/WFC_Gen/F_Position Structure") (SideToCheck :type "/Game/WFC_Gen/EWFCB_Side Enum" :default "NewEnumerator0"))
  (returns (bWasUpdated :type Boolean))
  (locals (Cell :type "/Game/WFC_Gen/WFCB Structure") (NextCell :type "/Game/WFC_Gen/WFCB Structure") (WFCB_TypesToCompare :type "Array of /Game/WFC_Gen/EWFCB_Type Enum") (bUpdated :type Boolean) (WFCB_TypesToOverride :type "Array of /Game/WFC_Gen/EWFCB_Type Enum"))
  (bind (_x _y) (break `/Game/WFC_Gen/F_Position` Pointer))
  (bind _newposition (`self.GetSidePosition` Pointer SideToCheck))
  (bind _wfcb_typestocompare (`local.WFCB_TypesToCompare`))
  (bind _size (`self.Size`))
  (bind _grid (`self.Grid`))
  (bind _wfcb_typestooverride (`local.WFCB_TypesToOverride`))
  (bind (_x_2 _y_2) (break `/Game/WFC_Gen/F_Position` _newposition))
  (bind (_block _entropy _possibletypes) (break `/Game/WFC_Gen/WFCB` (`local.NextCell`)))
  (bind (_block_2 _entropy_2 _possibletypes_2) (break `/Game/WFC_Gen/WFCB` (`local.NextCell`)))
  (bind _returnvalue (or (>= _x_2 _size) (>= _y_2 _size) (< _x_2 0) (< _y_2 0)))
  (bind _returnvalue_2 (select `bool` _returnvalue :`false` _newposition))
  (bind (_x_3 _y_3) (break `/Game/WFC_Gen/F_Position` _returnvalue_2))
  (if _returnvalue
    _
    (elif (not (`KismetArrayLibrary.Array_Contains` (`self.PointerPositions`) _returnvalue_2))
      (set `local.Cell` (`self.GetGridCell` _x _y _grid))
      (bind _output_get (set `local.NextCell` (`self.GetGridCell` _x_3 _y_3 _grid)))
      (if (== (`.Entropy_12_E6113C984C0211854CA30DA3145B3B74` (break `/Game/WFC_Gen/WFCB` _output_get)) 1)
        _
        (else
          (for _array_element (`.PossibleTypes_13_0D2B1D3F473FAEEDA1964AB5036C1E91` (break `/Game/WFC_Gen/WFCB` (`local.Cell`)))
            (for _array_element_2 (`self.GetTruthTable` SideToCheck (`KismetArrayLibrary.Array_Contains` (`.Side_9_14B6240F41DCB321D70966A273F46EE9` (break `/Game/WFC_Gen/WFCB_Type` (`|GetArrayItem` (`self.AllTypes`) (`KismetMathLibrary.Conv_ByteToInt` _array_element)))) SideToCheck))
              (`KismetArrayLibrary.Array_AddUnique` _wfcb_typestocompare _array_element_2)))
          (set `local.WFCB_TypesToOverride` _possibletypes_2)
          (for _array_element_3 _possibletypes_2
            (if (not (`KismetArrayLibrary.Array_Contains` _wfcb_typestocompare _array_element_3))
              (`KismetArrayLibrary.Array_RemoveItem` (`local.WFCB_TypesToOverride`) _array_element_3)
              (set `local.bUpdated` true)))
          (bind _structout (setmembers `/Game/WFC_Gen/WFCB` :`StructRef` (`local.NextCell`) :`Entropy` (`KismetArrayLibrary.Array_Length` _wfcb_typestooverride) :`PossibleTypes` _wfcb_typestooverride))
          (`KismetArrayLibrary.Array_Set` (`.Y_Blocks_8_E43C58594D4CAD8B76D849A3CB4CB618` (break `/Game/WFC_Gen/ARR_WFCB_2D` (`|GetArrayItem` (`self.Grid`) _x_3))) _y_3 _structout)
          (if (== (`KismetArrayLibrary.Array_Length` _possibletypes) 1)
            (`self.CollapseCell` _block (`|GetArrayItem` _possibletypes)))
          (return (`local.bUpdated`))))))
  (return (`local.bUpdated`)))

(fn `CollapseCell`
  (params (Cell :type "/Game/WFC_Gen/Blocks/BP_WFCB Object Reference") (CellType :type "/Game/WFC_Gen/EWFCB_Type Enum" :default "NewEnumerator0"))
  (bind (_x _y) (`/Game/WFC_Gen/Blocks/BP_WFCB.GetPosition` Cell))
  (bind _grid (`self.Grid`))
  (bind _structout (setmembers `/Game/WFC_Gen/WFCB` :`StructRef` (`self.GetGridCell` _x _y _grid) :`Entropy` 1 :`PossibleTypes` (`|MakeArray` CellType)))
  (`KismetArrayLibrary.Array_Set` (`.Y_Blocks_8_E43C58594D4CAD8B76D849A3CB4CB618` (break `/Game/WFC_Gen/ARR_WFCB_2D` (`|GetArrayItem` _grid _x))) _y _structout)
  (`self.Spawn` CellType Cell)
  (`KismetArrayLibrary.Array_RemoveItem` (`self.UnCollapsedCells`) Cell)
  (return))

(fn `CollapseRandomCell`
  (params (UnCollapsedCells :type "Array of /Game/WFC_Gen/Blocks/BP_WFCB Object Reference (by ref)"))
  (returns (CollapsedCell :type "/Game/WFC_Gen/Blocks/BP_WFCB Object Reference"))
  (locals (RandValue :type "/Game/WFC_Gen/Blocks/BP_WFCB Object Reference") (HighestEntropyValue :type Integer :default 20) (CellsToSelect :type "Array of /Game/WFC_Gen/Blocks/BP_WFCB Object Reference"))
  (bind _cellstoselect (`local.CellsToSelect`))
  (bind _returnvalue (- (`self.Size`) 1))
  (for _array_element UnCollapsedCells
    (bind (_x _y) (`/Game/WFC_Gen/Blocks/BP_WFCB.GetPosition` _array_element))
    (bind (_block _entropy) (break `/Game/WFC_Gen/WFCB` (`self.GetGridCell` _x _y (`self.Grid`))))
    (if (< _entropy (`local.HighestEntropyValue`))
      (set `local.HighestEntropyValue` _entropy)))
  (for _index (range (+ _returnvalue 1))
    (for _index_2 (range (+ _returnvalue 1))
      (bind (_block_2 _entropy_2) (break `/Game/WFC_Gen/WFCB` (`self.GetGridCell` _index _index_2 (`self.Grid`))))
      (if (== _entropy_2 (`local.HighestEntropyValue`))
        (`KismetArrayLibrary.Array_Add` (`local.CellsToSelect`) _block_2))))
  (bind _output_get (set `local.RandValue` (`|GetArrayItem` _cellstoselect (`KismetMathLibrary.RandomInteger` (`KismetArrayLibrary.Array_Length` _cellstoselect)))))
  (bind (_x_2 _y_2) (`/Game/WFC_Gen/Blocks/BP_WFCB.GetPosition` _output_get))
  (`self.CollapseCell` _output_get (`KismetArrayLibrary.Array_Random` (`.PossibleTypes_13_0D2B1D3F473FAEEDA1964AB5036C1E91` (break `/Game/WFC_Gen/WFCB` (`.Block (a copy)` (`self.GetGridCell` _x_2 _y_2 (`self.Grid`)))))))
  (return _output_get))

(fn `ConstructWFCB_Type`
  (params (WFCB_Type :type "/Game/WFC_Gen/EWFCB_Type Enum" :default "NewEnumerator0") (AccessibleSides :type "Array of /Game/WFC_Gen/EWFCB_Side Enum"))
  (returns (NewParam :type "/Game/WFC_Gen/WFCB_Type Structure"))
  (return (make `/Game/WFC_Gen/WFCB_Type` WFCB_Type AccessibleSides)))

(fn `GetGridCell`
  (params (X :type Integer) (Y :type Integer) (Grid :type "Array of /Game/WFC_Gen/ARR_WFCB_2D Structure"))
  (returns (`Block (a ref)` :type "/Game/WFC_Gen/WFCB Structure") (`Block (a copy)` :type "/Game/WFC_Gen/WFCB Structure"))
  (return (`|GetArrayItem` (`.Y_Blocks_8_E43C58594D4CAD8B76D849A3CB4CB618` (break `/Game/WFC_Gen/ARR_WFCB_2D` (`|GetArrayItem` Grid X))) Y) (`|GetArrayItem` (`.Y_Blocks_8_E43C58594D4CAD8B76D849A3CB4CB618` (break `/Game/WFC_Gen/ARR_WFCB_2D` (`|GetArrayItem` Grid X))) Y)))

(fn `GetInvertedEWFCB_SideType`
  (params (Side :type "/Game/WFC_Gen/EWFCB_Side Enum (by ref)"))
  (returns (InvertedSide :type "/Game/WFC_Gen/EWFCB_Side Enum"))
  (return (select `/Game/WFC_Gen/EWFCB_Side` Side :`NewEnumerator0` "NewEnumerator2" :`NewEnumerator1` "NewEnumerator3" :`NewEnumerator2` "NewEnumerator0" :`NewEnumerator3` "NewEnumerator1" :!type "/Game/WFC_Gen/EWFCB_Side Enum")))

(fn `GetLineWay`
  (params (Start :type "/Game/WFC_Gen/F_Position Structure") (End :type "/Game/WFC_Gen/F_Position Structure"))
  (returns (way :type "Array of /Game/WFC_Gen/F_Position Structure"))
  (locals (WayToReturn :type "Array of /Game/WFC_Gen/F_Position Structure"))
  (bind (_x _y) (break `/Game/WFC_Gen/F_Position` End))
  (bind (_x_2 _y_2) (break `/Game/WFC_Gen/F_Position` Start))
  (bind _returnvalue (< _y_2 _y))
  (bind _returnvalue_2 (< _x_2 _x))
  (bind _returnvalue_3 (`KismetMathLibrary.SelectInt` _y_2 _y _returnvalue))
  (bind _returnvalue_4 (`KismetMathLibrary.SelectInt` _x_2 _x _returnvalue_2))
  (bind _returnvalue_5 (`KismetMathLibrary.SelectInt` _y_2 _y (not _returnvalue)))
  (bind _returnvalue_6 (`KismetMathLibrary.SelectInt` _x_2 _x (not _returnvalue_2)))
  (if (== _x_2 _x)
    (for _index (range _returnvalue_3 (+ _returnvalue_5 1))
      (`KismetArrayLibrary.Array_Add` (`local.WayToReturn`) (make `/Game/WFC_Gen/F_Position` _x_2 (`KismetMathLibrary.SelectInt` _index (`KismetMathLibrary.FTrunc` (`KismetMathLibrary.MapRangeClamped` (`KismetMathLibrary.Conv_IntToDouble` _index) (`KismetMathLibrary.Conv_IntToDouble` _returnvalue_3) (`KismetMathLibrary.Conv_IntToDouble` _returnvalue_5) (`KismetMathLibrary.Conv_IntToDouble` _returnvalue_5) (`KismetMathLibrary.Conv_IntToDouble` _returnvalue_3))) _returnvalue))))
    (return (`local.WayToReturn`))
    (elif (== _y_2 _y)
      (for _index_2 (range _returnvalue_4 (+ _returnvalue_6 1))
        (`KismetArrayLibrary.Array_Add` (`local.WayToReturn`) (make `/Game/WFC_Gen/F_Position` (`KismetMathLibrary.SelectInt` _index_2 (`KismetMathLibrary.FTrunc` (`KismetMathLibrary.MapRangeClamped` (`KismetMathLibrary.Conv_IntToDouble` _index_2) (`KismetMathLibrary.Conv_IntToDouble` _returnvalue_4) (`KismetMathLibrary.Conv_IntToDouble` _returnvalue_6) (`KismetMathLibrary.Conv_IntToDouble` _returnvalue_6) (`KismetMathLibrary.Conv_IntToDouble` _returnvalue_4))) _returnvalue_2) _y_2)))
      (return (`local.WayToReturn`)))))

(fn `GetSideFromDirection`
  (params (Direction :type "/Game/WFC_Gen/F_Position Structure"))
  (returns (Side :type "/Game/WFC_Gen/EWFCB_Side Enum"))
  (bind (_x _y) (break `/Game/WFC_Gen/F_Position` Direction))
  (bind (_x_2 _y_2) (break `/Game/WFC_Gen/F_Position` Direction))
  (bind (_x_3 _y_3) (break `/Game/WFC_Gen/F_Position` Direction))
  (bind (_x_4 _y_4) (break `/Game/WFC_Gen/F_Position` Direction))
  (if (and (== _x_2 0) (== _y_2 1))
    (return "NewEnumerator2")
    (elif (and (== _x_3 1) (== _y_3 0))
      (return "NewEnumerator1")
      (elif (and (== _x_4 0) (== _y_4 -1))
        (return "NewEnumerator0")
        (elif (and (== _x -1) (== _y 0))
          (return "NewEnumerator3"))))))

(fn `GetSidePosition`
  (params (Position :type "/Game/WFC_Gen/F_Position Structure") (Side :type "/Game/WFC_Gen/EWFCB_Side Enum" :default "NewEnumerator0"))
  (returns (NewPosition :type "/Game/WFC_Gen/F_Position Structure"))
  (bind (_x _y) (break `/Game/WFC_Gen/F_Position` Position))
  (bind (_x_2 _y_2) (break `/Game/WFC_Gen/F_Position` Position))
  (bind (_x_3 _y_3) (break `/Game/WFC_Gen/F_Position` Position))
  (bind (_x_4 _y_4) (break `/Game/WFC_Gen/F_Position` Position))
  (return (select `/Game/WFC_Gen/EWFCB_Side` Side :`NewEnumerator0` (make `/Game/WFC_Gen/F_Position` _x_4 (+ _y_4 -1)) :`NewEnumerator1` (make `/Game/WFC_Gen/F_Position` (+ _x_2 1) _y_2) :`NewEnumerator2` (make `/Game/WFC_Gen/F_Position` _x (+ _y 1)) :`NewEnumerator3` (make `/Game/WFC_Gen/F_Position` (+ _x_3 -1) _y_3))))

(fn `GetTruthTable`
  (params (SideToConnect :type "/Game/WFC_Gen/EWFCB_Side Enum" :default "NewEnumerator0") (bConects :type Boolean))
  (returns (TruthTable :type "Array of /Game/WFC_Gen/EWFCB_Type Enum"))
  (return (select `bool` bConects :`false` (select `/Game/WFC_Gen/EWFCB_Side` SideToConnect :`NewEnumerator0` (`|MakeArray` "NewEnumerator1" "NewEnumerator2" "NewEnumerator5" "NewEnumerator9" "NewEnumerator19" "NewEnumerator20" "NewEnumerator21" "NewEnumerator23" :!type "/Game/WFC_Gen/EWFCB_Type Enum") :`NewEnumerator1` (`|MakeArray` "NewEnumerator2" "NewEnumerator4" "NewEnumerator6" "NewEnumerator8" "NewEnumerator19" "NewEnumerator20" "NewEnumerator21" "NewEnumerator22" :!type "/Game/WFC_Gen/EWFCB_Type Enum") :`NewEnumerator2` (`|MakeArray` "NewEnumerator3" "NewEnumerator4" "NewEnumerator5" "NewEnumerator10" "NewEnumerator19" "NewEnumerator21" "NewEnumerator22" "NewEnumerator23" :!type "/Game/WFC_Gen/EWFCB_Type Enum") :`NewEnumerator3` (`|MakeArray` "NewEnumerator1" "NewEnumerator3" "NewEnumerator6" "NewEnumerator7" "NewEnumerator19" "NewEnumerator20" "NewEnumerator22" "NewEnumerator23" :!type "/Game/WFC_Gen/EWFCB_Type Enum")) :`true` (select `/Game/WFC_Gen/EWFCB_Side` SideToConnect :`NewEnumerator0` (`|MakeArray` "NewEnumerator0" "NewEnumerator3" "NewEnumerator4" "NewEnumerator6" "NewEnumerator7" "NewEnumerator8" "NewEnumerator10" "NewEnumerator22" :!type "/Game/WFC_Gen/EWFCB_Type Enum") :`NewEnumerator1` (`|MakeArray` "NewEnumerator0" "NewEnumerator1" "NewEnumerator3" "NewEnumerator5" "NewEnumerator7" "NewEnumerator9" "NewEnumerator10" "NewEnumerator23" :!type "/Game/WFC_Gen/EWFCB_Type Enum") :`NewEnumerator2` (`|MakeArray` "NewEnumerator0" "NewEnumerator1" "NewEnumerator2" "NewEnumerator6" "NewEnumerator7" "NewEnumerator8" "NewEnumerator9" "NewEnumerator20" :!type "/Game/WFC_Gen/EWFCB_Type Enum") :`NewEnumerator3` (`|MakeArray` "NewEnumerator0" "NewEnumerator2" "NewEnumerator4" "NewEnumerator5" "NewEnumerator8" "NewEnumerator9" "NewEnumerator10" "NewEnumerator21" :!type "/Game/WFC_Gen/EWFCB_Type Enum")))))

(fn `Initialize`
  (params (AllTypes :type "Array of /Game/WFC_Gen/WFCB_Type Structure"))
  (bind _ealltypes (`self.EAllTypes`))
  (bind _grid (`self.Grid`))
  (bind _returnvalue (- (`self.Size`) 1))
  (bind _returnvalue_2 (- (`self.Size`) 1))
  (bind _returnvalue_3 (`KismetMathLibrary.Conv_IntToDouble` (+ (* _returnvalue 800) 800)))
  (set `self.AllTypes` AllTypes)
  (bind _enumvalue (foreach `/Game/WFC_Gen/EWFCB_Type` false)
    (:`LoopBody`
      (`KismetArrayLibrary.Array_Add` (`self.EAllTypes`) _enumvalue))
    (:`then`
      ;[0 0 0] X
      (for _index (range (+ _returnvalue_2 1))
        (bind _returnvalue_4 (`KismetArrayLibrary.Array_Add` _grid))
        ;;[0 0.0296 0.5365] Y
        (for _index_2 (range (+ _returnvalue_2 1))
          (bind _y_blocks (break `/Game/WFC_Gen/ARR_WFCB_2D` (`|GetArrayItem` _grid _returnvalue_4)))
          ;;;[0 0 0] Individual Block
          (bind _returnvalue_5 (`KismetArrayLibrary.Array_Add` _y_blocks))
          (bind _returnvalue_6 (`|SpawnActorFromClass` "/Game/WFC_Gen/Blocks/BP_WFCB.BP_WFCB_C" (`KismetMathLibrary.MakeTransform` (`KismetMathLibrary.MakeVector` (* _index 800.0) (* _index_2 800.0))) "Undefined" "OverrideRootScale" null null))
          (`/Game/WFC_Gen/Blocks/BP_WFCB.Initialize` _returnvalue_6 _index _index_2)
          (bind _structout (setmembers `/Game/WFC_Gen/WFCB` :`StructRef` (`|GetArrayItem` _y_blocks _returnvalue_5) :`Block` _returnvalue_6 :`Entropy` (`KismetArrayLibrary.Array_Length` _ealltypes) :`PossibleTypes` _ealltypes))
          (`KismetArrayLibrary.Array_Set` _y_blocks _returnvalue_5 _structout)))
      (for _array_element _grid
        (for _array_element_2 (`.Y_Blocks_8_E43C58594D4CAD8B76D849A3CB4CB618` (break `/Game/WFC_Gen/ARR_WFCB_2D` _array_element))
          (`KismetArrayLibrary.Array_Add` (`self.UnCollapsedCells`) (`.Block_6_8AF3130D42DC3D65C3CDCA9B9FFBBDAE` (break `/Game/WFC_Gen/WFCB` _array_element_2)))))
      (bind _enumvalue_2 (foreach `/Game/WFC_Gen/EWFCB_Side` false)
        (:`LoopBody`
          (for _index_3 (range (+ _returnvalue 1))
            (if (or (and (== _index_3 0) (`|EnumEquality` _enumvalue_2 "NewEnumerator3")) (and (== _index_3 18) (`|EnumEquality` _enumvalue_2 "NewEnumerator2")))
              (bind _returnvalue_7 (`KismetMathLibrary.Conv_IntToDouble` (* _index_3 800)))
              (bind _returnvalue_8 (`KismetMathLibrary.MakeTransform` (`KismetMathLibrary.MakeVector` (select `/Game/WFC_Gen/EWFCB_Side` _enumvalue_2 :`NewEnumerator0` _returnvalue_7 :`NewEnumerator1` _returnvalue_3 :`NewEnumerator2` _returnvalue_7 :`NewEnumerator3` -800.0) (select `/Game/WFC_Gen/EWFCB_Side` _enumvalue_2 :`NewEnumerator0` -800.0 :`NewEnumerator1` _returnvalue_7 :`NewEnumerator2` _returnvalue_3 :`NewEnumerator3` _returnvalue_7)) (select `/Game/WFC_Gen/EWFCB_Side` _enumvalue_2 :`NewEnumerator0` (struct :`Yaw` 90.0) :`NewEnumerator1` (struct :`Yaw` 180.0) :`NewEnumerator2` (struct :`Yaw` -90.0) :!type "Rotator Structure")))
              (`InstancedStaticMeshComponent.AddInstance` (`self.WFCB_HorizontalInstances`) _returnvalue_8 false)
              (else
                (`InstancedStaticMeshComponent.AddInstance` (`self.WFCB_EndInstances`) _returnvalue_8 false)))))
        (:`then`
          (return))))))

(fn `MovePointer`
  (params (SideToMoveTo :type "/Game/WFC_Gen/EWFCB_Side Enum" :default "NewEnumerator0") (Pointer :type "/Game/WFC_Gen/F_Position Structure (by ref)"))
  (`|VariableSetRef` Pointer (`self.GetSidePosition` Pointer SideToMoveTo))
  (return))

(fn `PreConstructGrid`
  (params (Way :type "Array of /Game/WFC_Gen/F_Position Structure"))
  (returns (WayToConstruct :type "Array of /Game/WFC_Gen/F_Position Structure"))
  (locals (PossibleTypes :type "Array of /Game/WFC_Gen/EWFCB_Type Enum"))
  (bind _possibletypes (`local.PossibleTypes`))
  (bind _grid (`self.Grid`))
  (bind _waytoconstruct (`self.WayToConstruct`))
  (for (_array_element _array_index) Way
    (bind _way (`self.GetLineWay` _array_element (`|GetArrayItem` Way (+ _array_index 1))))
    (for _array_element_2 _way
      (`KismetArrayLibrary.Array_AddUnique` (`self.WayToConstruct`) _array_element_2)))
  (for _index (range 1 (+ (- (`KismetArrayLibrary.Array_Length` _waytoconstruct) 2) 1))
    (`KismetArrayLibrary.Array_Clear` (`local.PossibleTypes`))
    (bind (_x _y) (break `/Game/WFC_Gen/F_Position` (`|GetArrayItem` _waytoconstruct (- _index 1))))
    (bind (_x_2 _y_2) (break `/Game/WFC_Gen/F_Position` (`|GetArrayItem` _waytoconstruct _index)))
    (bind _side (`self.GetSideFromDirection` (make `/Game/WFC_Gen/F_Position` (- _x _x_2) (- _y _y_2))))
    (bind (_x_3 _y_3) (break `/Game/WFC_Gen/F_Position` (`|GetArrayItem` _waytoconstruct (- _index -1))))
    (bind _side_2 (`self.GetSideFromDirection` (make `/Game/WFC_Gen/F_Position` (- _x_3 _x_2) (- _y_3 _y_2))))
    (for _array_element_3 (`self.AllTypes`)
      (bind (_type _side_3) (break `/Game/WFC_Gen/WFCB_Type` _array_element_3))
      (if (and (`KismetArrayLibrary.Array_Contains` _side_3 _side) (`KismetArrayLibrary.Array_Contains` _side_3 _side_2))
        (`KismetArrayLibrary.Array_Add` (`local.PossibleTypes`) _type)))
    (bind _structout (setmembers `/Game/WFC_Gen/WFCB` :`StructRef` (`self.GetGridCell` _x_2 _y_2 _grid) :`Entropy` (`KismetArrayLibrary.Array_Length` _possibletypes) :`PossibleTypes` _possibletypes))
    (`KismetArrayLibrary.Array_Set` (`.Y_Blocks_8_E43C58594D4CAD8B76D849A3CB4CB618` (break `/Game/WFC_Gen/ARR_WFCB_2D` (`|GetArrayItem` _grid _x_2))) _y_2 _structout))
  (return _waytoconstruct))

(fn `PreConstructGridUpdate`
  (params (WayToConstruct :type "Array of /Game/WFC_Gen/F_Position Structure"))
  (bind _returnvalue (- (`KismetArrayLibrary.Array_Length` WayToConstruct) 2))
  (for _index (range 1 (+ _returnvalue 1))
    (bind (_x _y) (break `/Game/WFC_Gen/F_Position` (`|GetArrayItem` WayToConstruct _index)))
    (bind (_block _entropy _possibletypes) (break `/Game/WFC_Gen/WFCB` (`.Block (a copy)` (`self.GetGridCell` _x _y (`self.Grid`)))))
    (`self.CollapseCell` _block (`KismetArrayLibrary.Array_Random` _possibletypes)))
  (for _index_2 (range 1 (+ _returnvalue 1))
    (`self.UpdateGrid` (`|GetArrayItem` WayToConstruct _index_2)))
  (return))

(fn `Spawn`
  (params (BlockType :type "/Game/WFC_Gen/EWFCB_Type Enum" :default "NewEnumerator0") (NewParam :type "/Game/WFC_Gen/Blocks/BP_WFCB Object Reference"))
  (bind (_x _y) (`/Game/WFC_Gen/Blocks/BP_WFCB.GetPosition` NewParam))
  (bind _wfcb_horizontalinstances (`self.WFCB_HorizontalInstances`))
  (bind _wfcb_endinstances (`self.WFCB_EndInstances`))
  (bind _wfcb_toprightinstances (`self.WFCB_TopRightInstances`))
  (bind _wfcb_trightinstances (`self.WFCB_TRightInstances`))
  (bind _returnvalue (select `/Game/WFC_Gen/EWFCB_Type` BlockType :`NewEnumerator0` (`self.WFCB_IntersectionInstances`) :`NewEnumerator1` _wfcb_toprightinstances :`NewEnumerator2` _wfcb_toprightinstances :`NewEnumerator3` _wfcb_toprightinstances :`NewEnumerator4` _wfcb_toprightinstances :`NewEnumerator5` _wfcb_horizontalinstances :`NewEnumerator6` _wfcb_horizontalinstances :`NewEnumerator7` _wfcb_trightinstances :`NewEnumerator8` _wfcb_trightinstances :`NewEnumerator9` _wfcb_trightinstances :`NewEnumerator10` _wfcb_trightinstances :`NewEnumerator20` _wfcb_endinstances :`NewEnumerator21` _wfcb_endinstances :`NewEnumerator22` _wfcb_endinstances :`NewEnumerator23` _wfcb_endinstances))
  (if (`|EnumInequality` BlockType "NewEnumerator19")
    (`InstancedStaticMeshComponent.AddInstance` _returnvalue (`KismetMathLibrary.MakeTransform` (`KismetMathLibrary.MakeVector` (`KismetMathLibrary.Conv_IntToDouble` (* _x 800)) (`KismetMathLibrary.Conv_IntToDouble` (* _y 800))) (select `/Game/WFC_Gen/EWFCB_Type` BlockType :`NewEnumerator1` (struct :`Yaw` -90.0) :`NewEnumerator3` (struct :`Yaw` 180.0) :`NewEnumerator4` (struct :`Yaw` 90.0) :`NewEnumerator6` (struct :`Yaw` 90.0) :`NewEnumerator7` (struct :`Yaw` 90.0) :`NewEnumerator8` (struct :`Yaw` -90.0) :`NewEnumerator9` (struct :`Yaw` 180.0) :`NewEnumerator20` (struct :`Yaw` -90.0) :`NewEnumerator22` (struct :`Yaw` 90.0) :`NewEnumerator23` (struct :`Yaw` 180.0) :!type "Rotator Structure")) false)
    (`PrimitiveComponent.SetMaterial` _returnvalue 0 "/Game/Models/Layout/ModularMaze/Walls.Walls")
    (return)
    (else
      (return))))

(fn `UpdateGrid`
  (params (Pointer :type "/Game/WFC_Gen/F_Position Structure (by ref)"))
  (locals (Pointer :type "/Game/WFC_Gen/F_Position Structure") (CheckedAndUpdatedCells :type "Array of /Game/WFC_Gen/F_Position Structure"))
  (bind _pointerpositions (`self.PointerPositions`))
  (bind _pointer (`local.Pointer`))
  (bind _returnvalue (`KismetArrayLibrary.Array_LastIndex` _pointerpositions))
  (`KismetArrayLibrary.Array_AddUnique` (`self.PointerPositions`) Pointer)
  (bind _enumvalue (foreach `/Game/WFC_Gen/EWFCB_Side` false)
    (:`LoopBody`
      (bind _bwasupdated (`self.CheckAndUpdateCell` (`local.Pointer`) _enumvalue))
      (if _bwasupdated
        (`self.MovePointer` _enumvalue (`local.Pointer`))
        (`self.UpdateGrid` (`local.Pointer`))))
    (:`then`
      (if (> (`KismetArrayLibrary.Array_Length` _pointerpositions) 1)
        (`KismetArrayLibrary.Array_Remove` _pointerpositions _returnvalue)
        (`|VariableSetRef` _pointer (`|GetArrayItem` _pointerpositions _returnvalue))
        (`self.UpdateGrid` _pointer)
        (else
          (return))))))

(fn `UserConstructionScript`)