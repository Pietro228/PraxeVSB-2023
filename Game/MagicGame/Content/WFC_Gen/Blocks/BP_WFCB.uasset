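; Grid block for what appears to be a Wave Function Collapse generator, storing its X/Y cell position.
; Spawn maps a block type to a piece Blueprint and places it at the block's location.
; Corner, straight and T-junction variants each reuse one class per shape, rotated in 90-degree steps.
; The C-prefixed and Empty types have no class assigned.
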(fn `GetPosition`
  (returns (X :type Integer) (Y :type Integer))
  (return (`self.X`) (`self.Y`)))

(fn `Initialize`
  (params (PosX :type Integer) (PosY :type Integer))
  (set `self.X` PosX)
  (set `self.Y` PosY))

(fn `Spawn`
  (params (BlockType :type "/Game/WFC_Gen/EWFCB_Type Enum" :default "NewEnumerator0"))
  (`|SpawnActorFromClass` (select `/Game/WFC_Gen/EWFCB_Type` BlockType :`NewEnumerator0` "/Game/WFC_Gen/Blocks/BP_WFCB_Intersection.BP_WFCB_Intersection_C" :`NewEnumerator1` "/Game/WFC_Gen/Blocks/BP_WFCB_TopRight.BP_WFCB_TopRight_C" :`NewEnumerator2` "/Game/WFC_Gen/Blocks/BP_WFCB_TopRight.BP_WFCB_TopRight_C" :`NewEnumerator3` "/Game/WFC_Gen/Blocks/BP_WFCB_TopRight.BP_WFCB_TopRight_C" :`NewEnumerator4` "/Game/WFC_Gen/Blocks/BP_WFCB_TopRight.BP_WFCB_TopRight_C" :`NewEnumerator5` "/Game/WFC_Gen/Blocks/BP_WFCB_Horizontal.BP_WFCB_Horizontal_C" :`NewEnumerator6` "/Game/WFC_Gen/Blocks/BP_WFCB_Horizontal.BP_WFCB_Horizontal_C" :`NewEnumerator7` "/Game/WFC_Gen/Blocks/BP_WFCB_TRight.BP_WFCB_TRight_C" :`NewEnumerator8` "/Game/WFC_Gen/Blocks/BP_WFCB_TRight.BP_WFCB_TRight_C" :`NewEnumerator9` "/Game/WFC_Gen/Blocks/BP_WFCB_TRight.BP_WFCB_TRight_C" :`NewEnumerator10` "/Game/WFC_Gen/Blocks/BP_WFCB_TRight.BP_WFCB_TRight_C" :!type "Actor Class Reference") (`KismetMathLibrary.MakeTransform` (`SceneComponent.K2_GetComponentLocation` (`self.DefaultSceneRoot`)) (select `/Game/WFC_Gen/EWFCB_Type` BlockType :`NewEnumerator1` (struct :`Yaw` -90.0) :`NewEnumerator3` (struct :`Yaw` 180.0) :`NewEnumerator4` (struct :`Yaw` 90.0) :`NewEnumerator6` (struct :`Yaw` 90.0) :`NewEnumerator7` (struct :`Yaw` 180.0) :`NewEnumerator9` (struct :`Yaw` -90.0) :`NewEnumerator10` (struct :`Yaw` 90.0) :!type "Rotator Structure")) "Undefined" "OverrideRootScale" null null))

(fn `UserConstructionScript`)